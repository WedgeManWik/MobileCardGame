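; BP_Card_FiredUp is a card actor for a single-target ability.
; Activate binds ExecAbility to the player controller's BC_TargetSelector and requests one target.
; ExecAbility only plays a montage on the player character's skeletal mesh, and AffectActors is empty.
; The logic that launches BP_FireBall at each target and reports the card as used is disconnected, so it never runs.
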(event `/Game/CardActors/BI_Card.Activate`
  (bind _returnvalue (`self.GetComponentByClass` (`GameplayStatics.GetPlayerController` 0) "/Game/Components/BC_TargetSelector.BC_TargetSelector_C"))
  (add `/Game/Components/BC_TargetSelector.OnDesiredNumTargetsSelected` _returnvalue (delegate `ExecAbility`))
  (`/Game/Components/BC_TargetSelector.SelectTargets` _returnvalue 1))

(event `ExecAbility`
  (params (Targets :type "Array of Actor Object Reference (by ref)"))
  (`|PlayMontage` (`self.GetComponentByClass` (`GameplayStatics.GetPlayerCharacter` 0) "/Script/Engine.SkeletalMeshComponent")))

(event `/Game/CardActors/BI_Card.AffectActors`
  (params (AffectedTargets :type "Array of Actor Object Reference (by ref)")))

(fn `UserConstructionScript`
  (`parent.UserConstructionScript`))