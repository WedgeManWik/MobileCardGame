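; BP_Card is a card actor that displays its card information through a widget component.
; The construction script calls InitialiseCard, which creates a WB_Card widget from CardInfo, stores it and assigns it to the CardWidget component.
; GetCardWidget exposes the stored widget, while Activate and AffectActors are empty stubs with no card effect in this Blueprint.
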(event `self.ReceiveBeginPlay`)

(event `InitialiseCard`
  (bind _returnvalue (`|CreateWidget` "/Game/CardUi/WB_Card.WB_Card_C" null (`self.CardInfo`)))
  (bind _output_get (set `self.Widget` _returnvalue))
  (`WidgetComponent.SetWidget` (`self.CardWidget`) _output_get))

(event `/Game/CardActors/BI_Card.Activate`)

(fn `AffectActors`
  (params (AffectedTargets :type "Array of Actor Object Reference (by ref)"))
  (return))

(fn `GetCardWidget`
  (returns (`Card Widget` :type "/Game/CardUi/WB_Card Object Reference"))
  (return (`self.Widget`)))

(fn `UserConstructionScript`
  (`self.InitialiseCard`))