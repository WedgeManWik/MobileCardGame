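; Player controller for a turn-based card game with touch input, managing the card HUD, input modes and enemy target selection.
; Turn events enable or disable the card HUD, and ending a turn notifies the GameMode.
; During selection, touches toggle BI_Enemy actors in a capped target list while WB_SelectTargets is shown.
; Confirming sends an Action.TargetsSet gameplay event to the pawn; GetSelectedTargets exposes the list, while GetCardBeingUsed returns only None.
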(event `self.ReceiveBeginPlay`
  (`EnhancedInputSubsystemInterface.AddMappingContext` (subsystem `EnhancedInputLocalPlayerSubsystem`) "/Game/Player/Input/IMC_Player.IMC_Player" 0 (struct))
  (bind _returnvalue (`|CreateWidget` "/Game/Cards/WB_CardHUD.WB_CardHUD_C" self))
  (bind _output_get (set `self.CardHUD` _returnvalue))
  (`UserWidget.AddToViewport` _output_get 0)
  (`WidgetBlueprintLibrary.SetInputMode_UIOnlyEx` self _output_get)
  (`GameplayStatics.GetActorOfClass` "/Script/Engine.CameraActor"))

(event `EnhancedInput|/Game/Player/Input/IA_Touch`
  (params (ActionValue :type Boolean) (ElapsedSeconds :type "Float (double-precision)") (TriggeredSeconds :type "Float (double-precision)") (InputAction :type "InputAction Object Reference" :default "/Game/Player/Input/IA_Touch.IA_Touch"))
  (bind _targetsselected (`self.TargetsSelected`))
  (bind _targetsselected_2 (`self.TargetsSelected`))
  (bind (_bblockinghit _binitialoverlap _time _distance _location _impactpoint _normal _impactnormal _physmat _hitactor) (`GameplayStatics.BreakHitResult` (`self.GetHitResultUnderFingerByChannel` "Touch1" "TraceTypeQuery2")))
  (bind _returnvalue (`KismetArrayLibrary.Array_Find` _targetsselected _hitactor))
  (:`Started`
    (if (`KismetSystemLibrary.DoesImplementInterface` _hitactor "/Game/Enemies/BI_Enemy.BI_Enemy_C")
      (bind _isturn (message `/Game/TopDown/Blueprints/BI_CardGameMode.IsMyTurn` (`GameplayStatics.GetGameMode`) self))
      (if (and _isturn (`self.IsSelectingTargets`))
        (if (>= _returnvalue 0)
          (`KismetArrayLibrary.Array_Remove` _targetsselected_2 _returnvalue)
          (if (> (`KismetArrayLibrary.Array_Length` _targetsselected_2) 0) :!label _label
            (`/Game/Cards/WB_SelectTargets.SelectedTargets` (`self.SelectTargetsHUD`)))
          (elif (< (`KismetArrayLibrary.Array_Length` _targetsselected) (`self.Max Num Targets`))
            (`KismetArrayLibrary.Array_Add` _targetsselected_2 _hitactor)
            (goto _label)))))))

(event `/Game/Cards/BI_CardUser.SelectTargetsToUseOnCard`
  (params (MaxNumTargets :type Integer))
  (set `self.IsSelectingTargets` true)
  (set `self.Max Num Targets` MaxNumTargets)
  (`KismetArrayLibrary.Array_Clear` (`self.TargetsSelected`))
  (bind _returnvalue (`|CreateWidget` "/Game/Cards/WB_SelectTargets.WB_SelectTargets_C" self))
  (bind _output_get (set `self.SelectTargetsHUD` _returnvalue))
  (add `/Game/Cards/WB_SelectTargets.OnTargetsConfirmed` _output_get (delegate `TargetsConfirmed`))
  (`UserWidget.AddToViewport` _output_get 0)
  (`WidgetBlueprintLibrary.SetInputMode_GameAndUIEx` self (`self.SelectTargetsHUD`)))

(event `TargetsConfirmed`
  (bind _returnvalue (`self.K2_GetPawn`))
  (set `self.IsSelectingTargets` false)
  (`Widget.RemoveFromParent` (`self.SelectTargetsHUD`))
  (`AbilitySystemBlueprintLibrary.SendGameplayEventToActor` _returnvalue (struct :`TagName` "Action.TargetsSet") (make `GameplayEventData` (struct :`TagName` "Action.TargetsSet") null _returnvalue)))

(event `/Game/Player/Blueprints/BI_Player.SetInputModeUIOnly`
  (`WidgetBlueprintLibrary.SetInputMode_UIOnlyEx` self (`self.CardHUD`)))

(event `/Game/Player/Blueprints/BI_Player.SetInputModeGameOnly`
  (`WidgetBlueprintLibrary.SetInputMode_GameOnly` self))

(event `/Game/Cards/BI_CardUser.CardHasBeenUsed`
  (`/Game/Cards/WB_CardHand.CardHasBeenUsed` (`/Game/Cards/WB_CardHUD.WB_CardHand` (`self.CardHUD`))))

(event `/Game/Cards/BI_CardUser.StartTurn`
  (bind _cardhud (`self.CardHUD`))
  (`/Game/Cards/WB_CardHUD.Enable` _cardhud)
  (`WidgetBlueprintLibrary.SetInputMode_UIOnlyEx` self _cardhud))

(event `/Game/Cards/BI_CardUser.EndTurn`
  (`/Game/Cards/WB_CardHUD.Disable` (`self.CardHUD`))
  (message `/Game/TopDown/Blueprints/BI_CardGameMode.FinishedTurn` (`GameplayStatics.GetGameMode`)))

(fn `GetCardBeingUsed`
  (returns (CardID :type Name) (WidgetRef :type "/Game/Cards/WB_Card Object Reference"))
  (return "None" null))

(fn `GetSelectedTargets`
  (returns (Targets :type "Array of Actor Object Reference"))
  (return (`self.TargetsSelected`)))

(fn `UserConstructionScript`)