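; BP_PlayerCharacter is the player character for card-based play, tracking the ID of the card being used and exposing it through a getter.
; Target selection and retrieval of selected targets are forwarded to its controller through message calls, so the character holds no targeting logic.
; Health and mana change events only print current and maximum values from the AttributeSet to the screen.
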(event `/Game/Cards/BI_CardUser.SelectTargetsToUseOnCard`
  (params (MaxNumTargets :type Integer))
  (message `/Game/Cards/BI_CardUser.SelectTargetsToUseOnCard` (`self.GetController`) MaxNumTargets))

(event `/Game/Cards/BI_CardUser.SetCardBeingUsed`
  (params (CardID :type Name))
  (set `self.CardBeingUsed` CardID))

(event `self.OnHealthChanged`
  (params (OldValue :type "Float (single-precision)") (NewValue :type "Float (single-precision)"))
  (bind (_maxhealth_basevalue _maxhealth_currentvalue) (break `GameplayAttributeData` (`GAAttributeSet.MaxHealth` (`self.AttributeSet`))))
  (`KismetSystemLibrary.PrintString` (`KismetStringLibrary.Concat_StrStr` "Health: " (`KismetStringLibrary.Conv_DoubleToString` NewValue) "/" (`KismetStringLibrary.Conv_DoubleToString` _maxhealth_currentvalue))))

(event `self.OnManaChanged`
  (params (OldValue :type "Float (single-precision)") (NewValue :type "Float (single-precision)"))
  (bind (_maxmana_basevalue _maxmana_currentvalue) (break `GameplayAttributeData` (`GAAttributeSet.MaxMana` (`self.AttributeSet`))))
  (`KismetSystemLibrary.PrintString` (`KismetStringLibrary.Concat_StrStr` "Mana: " (`KismetStringLibrary.Conv_DoubleToString` NewValue) "/" (`KismetStringLibrary.Conv_DoubleToString` _maxmana_currentvalue))))

(fn `GetCardBeingUsed`
  (returns (CardID :type Name))
  (return (`self.CardBeingUsed`)))

(fn `GetSelectedTargets`
  (returns (Targets :type "Array of Actor Object Reference"))
  (bind _targets (message `/Game/Cards/BI_CardUser.GetSelectedTargets` (`self.GetController`)))
  (return _targets))

(fn `UserConstructionScript`)