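; Gameplay ability that instantly applies an attribute-changing status effect to selected targets, intended to last until the end of each target's turn.
; On activation it gets the selected targets from the owning actor and adds a BC_AddToAttributeForNumTurns component to each with a one-turn count, then finishes.
; The component receives the ability's change amount, status effect and GameplayEffect class, with the owner as causer, leaving duration handling to that component.
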(event `self.K2_ActivateAbility`
  (`parent.K2_ActivateAbility`)
  (bind _targets (message `/Game/Cards/BI_CardUser.GetSelectedTargets` (`self.GetOwningActorFromActorInfo`)))
  (for _array_element _targets
    (`|AddComponentByClass` _array_element "/Game/Components/BC_AddToAttributeForNumTurns.BC_AddToAttributeForNumTurns_C" (`self.Attribute Change By`) 0 null (`self.Status Effect`) _array_element (`self.GetOwningActorFromActorInfo`) "NewEnumerator0" "NewEnumerator0" (`self.Gameplay Effect Class`) 0.0 0.0 1))
  (`self.FinishAbility`))