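; GA_DamageGA is a Gameplay Ability that provides a reusable DamageActor function for damaging a target through GAS.
; DamageActor builds an outgoing spec from the supplied gameplay effect class and sets the absolute Damage value as a SetByCaller magnitude under Event.Damage.
; The owner's ability system component then applies that spec to the target actor's component.
; The event graph holds only disabled placeholder events, with no activation logic.
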(fn `DamageActor`
  (params (Actor :type "Actor Object Reference") (DamageType :type "GameplayEffect Class Reference"))
  (bind _returnvalue (`self.GetAbilitySystemComponentFromActorInfo`))
  (bind _returnvalue_2 (`AbilitySystemBlueprintLibrary.AssignTagSetByCallerMagnitude` (`AbilitySystemComponent.MakeOutgoingSpec` :`self` _returnvalue :`GameplayEffectClass` DamageType) (struct :`TagName` "Event.Damage") (`KismetMathLibrary.Abs` (`self.Damage`))))
  (`AbilitySystemComponent.BP_ApplyGameplayEffectSpecToTarget` _returnvalue _returnvalue_2 (`AbilitySystemBlueprintLibrary.GetAbilitySystemComponent` Actor)))