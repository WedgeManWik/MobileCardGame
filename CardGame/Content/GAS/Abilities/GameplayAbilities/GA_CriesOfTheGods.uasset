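; GA_CriesOfTheGods is a card-based gameplay ability that spends mana to strike every enemy from above, applying damage to each one hit.
; It runs the parent activation once per enemy, setting that enemy as Target and the spawn location high overhead.
; Each Event.TargetHit applies GE_Damage with a negative set-by-caller magnitude to the payload actor and decrements a hit counter.
; When the counter runs out, it sends Event.AbilityFinished to the owner.
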(event `self.K2_ActivateAbility`
  (bind _returnvalue (`self.GetAbilitySystemComponentFromActorInfo`))
  (`self.InitialiseCard`)
  (`self.UseCardMana`)
  (bind _enemies (message `/Game/Cards/BI_CardUser.GetAllEnemies` (`self.GetOwningActorFromActorInfo`)))
  (set `self.NumHitsLeft` (`KismetArrayLibrary.Array_Length` _enemies))
  (for _array_element _enemies
    (set `self.Target` _array_element)
    (set `self.SpawnLocation` (+ (`Actor.K2_GetActorLocation` _array_element) (0.0 0.0 1000.0)))
    (`parent.K2_ActivateAbility`))
  (bind (_asynctaskproxy _payload) (`AbilityAsync_WaitGameplayEvent.WaitGameplayEventToActor` (`self.GetOwningActorFromActorInfo`) (struct :`TagName` "Event.TargetHit"))
    (:`EventReceived`
      (bind _asactor (cast `Actor` (`.OptionalObject` (break `GameplayEventData` _payload))))
      (bind _returnvalue_2 (`AbilitySystemBlueprintLibrary.AssignTagSetByCallerMagnitude` (`AbilitySystemComponent.MakeOutgoingSpec` :`self` _returnvalue :`GameplayEffectClass` "/Game/GAS/Effects/GE_Damage.GE_Damage_C") (struct :`TagName` "Event.Damage") (* (`KismetMathLibrary.Abs` (`self.Damage`)) -1.0)))
      (`AbilitySystemComponent.BP_ApplyGameplayEffectSpecToTarget` _returnvalue _returnvalue_2 (`AbilitySystemBlueprintLibrary.GetAbilitySystemComponent` _asactor))
      (bind _result (`/Engine/EditorBlueprintResources/StandardMacros.DecrementInt` (`self.NumHitsLeft`))
        (:`  `
          (if (<= _result 0)
            (`AbilitySystemBlueprintLibrary.SendGameplayEventToActor` (`self.GetOwningActorFromActorInfo`) (struct :`TagName` "Event.AbilityFinished"))))))))