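; GA_FireAbility is a card-based Gameplay Ability for a fire action on a selected target.
; It initialises the card, runs GA_SelectTargets once, then waits for the TargetsSet event before spending card mana.
; It stores the first target and the owner's location, starts listening for TargetHit, then calls the parent activation.
; A hit sends AbilityFinished to the owner; the montage branch is unconnected.
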(event `self.K2_ActivateAbility`
  (bind _returnvalue (`self.GetOwningActorFromActorInfo`))
  (`self.InitialiseCard`)
  (`AbilitySystemComponent.K2_GiveAbilityAndActivateOnce` (`self.GetAbilitySystemComponentFromActorInfo`) "/Game/GAS/Abilities/GA_SelectTargets.GA_SelectTargets_C" 1 -1)
  (`AbilityTask_WaitGameplayEvent.WaitGameplayEvent` (struct :`TagName` "Action.TargetsSet") null true
    (:`EventReceived`
      (`self.UseCardMana`)
      (bind _targets (message `/Game/Cards/BI_CardUser.GetSelectedTargets` _returnvalue))
      (set `self.Target` (`|GetArrayItem` _targets))
      (set `self.SpawnLocation` (`Actor.K2_GetActorLocation` _returnvalue))
      (`AbilityAsync_WaitGameplayEvent.WaitGameplayEventToActor` (`self.GetOwningActorFromActorInfo`) (struct :`TagName` "Event.TargetHit")
        (:`then`
          (`parent.K2_ActivateAbility`))
        (:`EventReceived`
          (`AbilitySystemBlueprintLibrary.SendGameplayEventToActor` (`self.GetOwningActorFromActorInfo`) (struct :`TagName` "Event.AbilityFinished")))))))

(event `self.K2_OnEndAbility`
  (params (bWasCancelled :type Boolean))
  (`parent.K2_OnEndAbility` bWasCancelled))