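; BP_BaseProjectile is a base projectile actor for GAS abilities that damages actors it overlaps.
; OverlappedActor accepts only actors other than its owner that are in the Targets list, returning whether the hit counted.
; On a hit, the owner's Ability System Component applies GE_Damage to the target, passing Damage as a SetByCaller magnitude under Event.Damage.
; The owner then receives an Event.TargetHit gameplay event.
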(fn `OverlappedActor`
  (params (Actor :type "Actor Object Reference"))
  (returns (HitTarget :type Boolean))
  (bind _returnvalue (`self.GetOwner`))
  (bind _returnvalue_2 (`AbilitySystemBlueprintLibrary.GetAbilitySystemComponent` _returnvalue))
  (if (and (!= Actor _returnvalue) (!= (`KismetArrayLibrary.Array_Find` (`self.Targets`) Actor) -1))
    (bind _returnvalue_3 (`AbilitySystemBlueprintLibrary.AssignTagSetByCallerMagnitude` (`AbilitySystemComponent.MakeOutgoingSpec` :`self` _returnvalue_2 :`GameplayEffectClass` "/Game/GAS/Effects/GE_Damage.GE_Damage_C") (struct :`TagName` "Event.Damage") (`self.Damage`)))
    (`AbilitySystemComponent.BP_ApplyGameplayEffectSpecToTarget` _returnvalue_2 _returnvalue_3 (`AbilitySystemBlueprintLibrary.GetAbilitySystemComponent` Actor))
    (`AbilitySystemBlueprintLibrary.SendGameplayEventToActor` _returnvalue (struct :`TagName` "Event.TargetHit"))
    (return true)
    (else
      (return false))))

(fn `UserConstructionScript`)