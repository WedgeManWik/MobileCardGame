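; Ability actor for the Gameplay Ability System that reports whether it reaches an assigned target.
; SetTargettoHit stores the target, and OverlappedActor checks a supplied actor against it, excluding the owner.
; A match sends an Event.TargetHit gameplay event to the owner, carrying the target, and returns true.
; Destruction always fires the MissedTarget dispatcher, and no overlap event here calls the check itself.
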(event `/Game/GAS/Abilities/AbilityActors/BI_AbilityActor.SetTargetToHit`
  (params (Target :type "Actor Object Reference"))
  (set `self.Target` Target))

(event `self.ReceiveDestroyed`
  (`self.MissedTarget`))

(fn `OverlappedActor`
  (params (Actor :type "Actor Object Reference"))
  (returns (HitTarget :type Boolean))
  (bind _returnvalue (`self.GetOwner`))
  (bind _target (`self.Target`))
  (if (and (!= Actor _returnvalue) (== Actor _target))
    (`AbilitySystemBlueprintLibrary.SendGameplayEventToActor` _returnvalue (struct :`TagName` "Event.TargetHit") (make `GameplayEventData` (struct :`TagName` "Event.TargetHit") null null _target))
    (return true)
    (else
      (return false))))

(fn `UserConstructionScript`)