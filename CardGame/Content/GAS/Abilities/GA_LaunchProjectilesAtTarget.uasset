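; Card-driven gameplay ability that launches one projectile from the owning actor at each selected target.
; Targets come from the owner via message call; each projectile spawns facing its target and receives the full target list.
; Target-hit gameplay events and projectile miss callbacks share one counter.
; When the counter reaches the card's maximum affected targets, the ability sends an AbilityFinished event to the owner.
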(event `self.K2_ActivateAbility`
  (bind _returnvalue (`self.GetOwningActorFromActorInfo`))
  (bind (_cardinfo_name _cardinfo_image _cardinfo_description _cardinfo_backgroundcolour _cardinfo_abilities _cardinfo_manacost _cardinfo_cardid _cardinfo_nummaxtargetsaffected) (break `/Game/Cards/S_CardInfo` (`self.CardInfo`)))
  (bind _returnvalue_2 (`Actor.K2_GetActorLocation` _returnvalue))
  (`parent.K2_ActivateAbility`)
  (bind _targets (message `/Game/Cards/BI_CardUser.GetSelectedTargets` _returnvalue))
  (for _array_element _targets
    (bind _returnvalue_3 (`|SpawnActorFromClass` (`self.ProjectileClass`) (`KismetMathLibrary.MakeTransform` _returnvalue_2 (`KismetMathLibrary.FindLookAtRotation` _returnvalue_2 (`Actor.K2_GetActorLocation` _array_element))) "Undefined" "MultiplyWithRoot" (`self.GetOwningActorFromActorInfo`) null))
    (message `/Game/GAS/Abilities/AbilityActors/BI_AbilityActor.SetTargetsToHit` _returnvalue_3 _targets)
    (add `/Game/GAS/Abilities/AbilityActors/BP_AbilityActor.MissedTarget` _returnvalue_3 (delegate `MissedTarget`)))
  (`AbilityTask_WaitGameplayEvent.WaitGameplayEvent` (struct :`TagName` "Event.TargetHit") null
    (:`EventReceived`
      (bind _result (`/Engine/EditorBlueprintResources/StandardMacros.IncrementInt` (`self.HitCounter`) :!label _label)
        (:`  `
          (if (>= _result _cardinfo_nummaxtargetsaffected)
            (`AbilitySystemBlueprintLibrary.SendGameplayEventToActor` (`self.GetOwningActorFromActorInfo`) (struct :`TagName` "Event.AbilityFinished"))))))))

(event `MissedTarget`
  (goto _label))

(event `self.K2_OnEndAbility`
  (params (bWasCancelled :type Boolean))
  (`parent.K2_OnEndAbility` bWasCancelled))