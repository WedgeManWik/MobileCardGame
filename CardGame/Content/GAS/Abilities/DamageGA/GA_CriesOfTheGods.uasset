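; GA_CriesOfTheGods is a mana-costing card damage ability that rains projectiles from above onto every enemy.
; On the montage notify it fetches all enemies and launches a set number of projectiles at each, using the parent ability's launch logic.
; Spawn points are randomized in a box above each target, higher for each successive enemy.
; A countdown of expected hits drops on each hit or miss and finishes the ability at zero.
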(event `self.K2_ActivateAbility`
  (`parent.K2_ActivateAbility`)
  (`self.UseCardMana`)
  (`self.WaitForTargetHit`)
  (`self.PlayMontageAndWaitForNotify` "NewEnumerator0"))

(event `self.MontageNotify`
  (bind _enemies (message `/Game/Cards/BI_CardUser.GetAllEnemies` (`self.GetOwningActorFromActorInfo`)))
  (set `self.NumHitsLeft` (* (`KismetArrayLibrary.Array_Length` _enemies) (`self.NumProjectilesToSpawn`)))
  (for (_array_element _array_index) _enemies
    (set `self.Target` _array_element)
    (for _ (range 1 (+ (`self.NumProjectilesToSpawn`) 1))
      (set `self.SpawnLocation` (`KismetMathLibrary.RandomPointInBoundingBox` (+ (`Actor.K2_GetActorLocation` (`self.Target`)) (`KismetMathLibrary.MakeVector` 0.0 0.0 (+ (* _array_index 500) 1000))) (500.0 500.0 500.0)))
      (`self.Launch Damaging Projectile at Target` null))))

(event `self.MontageFinished`)

(event `self.TargetHit`
  (params (Actor :type "Actor Object Reference"))
  (`parent.TargetHit` Actor)
  (`self.RegisterHit`))

(event `RegisterHit`
  (bind _result (`/Engine/EditorBlueprintResources/StandardMacros.DecrementInt` (`self.NumHitsLeft`))
    (:`  `
      (if (== _result 0)
        (`self.FinishAbility`)))))

(fn `Projectile Missed Target`
  (`parent.Projectile Missed Target`)
  (`self.RegisterHit`))