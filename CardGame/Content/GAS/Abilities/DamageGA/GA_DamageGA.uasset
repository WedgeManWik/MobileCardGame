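; Base card-driven GAS damage ability that attacks the owner's selected targets one after another, with an empty AttackTarget event as the apparent hook for children.
; MontageFinished or a MissedTarget gameplay event advances to the next target, finishing the ability after the last.
; TargetHit gameplay events apply the DamageType effect, using damage read from card stats by ability level.
; Helpers rotate the player controller, or the actor without one, for aiming.
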(event `self.InitialiseCardStats`
  (bind (_cardinfo_name _cardinfo_image _cardinfo_description _cardinfo_backgroundcolour _cardinfo_abilities) (break `/Game/Cards/S_CardInfo` (`self.CardInfo`)))
  (set `self.Damage` (`|GetArrayItem` (`.Amounts_13_261E98044149E635A2EF1EB1BF0F7855` (break `/Game/Cards/S_GA_Details` (`|GetArrayItem` _cardinfo_abilities (`self.GetAbilityLevel`)))))))

(event `self.K2_ActivateAbility`
  (`parent.K2_ActivateAbility`)
  (`AbilityTask_WaitGameplayEvent.WaitGameplayEvent` (struct :`TagName` "Event.MissedTarget") null
    (:`EventReceived`
      (`self.MissedTarget`))))

(event `FocusOnTarget`
  (bind (_returnvalue_owneractor _returnvalue_avataractor _returnvalue_playercontroller) (break `GameplayAbilityActorInfo` (`self.GetActorInfo`)))
  (bind _returnvalue (`KismetMathLibrary.FindLookAtRotation` (`Actor.K2_GetActorLocation` _returnvalue_owneractor) (`Actor.K2_GetActorLocation` (`self.Target`))))
  (`/Engine/EditorBlueprintResources/StandardMacros.IsValid` _returnvalue_playercontroller
    (:`Is Valid`
      (`Controller.SetControlRotation` _returnvalue_playercontroller _returnvalue))
    (:`Is Not Valid`
      (`Actor.K2_SetActorRotation` _returnvalue_owneractor _returnvalue true))))

(event `MissedTarget`
  (`/Engine/EditorBlueprintResources/StandardMacros.IncrementInt` (`self.TargetIndex`)
    (:`  `
      (`self.AttackNextTarget`))))

(event `StartAttack`
  (`self.WaitForTargetHit`)
  (`self.AttackNextTarget`))

(event `AttackNextTarget`
  (bind _targets (message `/Game/Cards/BI_CardUser.GetSelectedTargets` (`self.GetOwningActorFromActorInfo`)))
  (bind _output_get (set `self.NumTargetsToHit` (`KismetArrayLibrary.Array_Length` _targets)))
  (if (< (`self.TargetIndex`) _output_get)
    (set `self.Target` (`|GetArrayItem` _targets (`self.TargetIndex`)))
    (`self.AttackTarget`)
    (else
      (`self.FinishAbility`))))

(event `SetFocusRotation`
  (params (NewRotation :type "Rotator Structure (by ref)"))
  (bind (_returnvalue_owneractor _returnvalue_avataractor _returnvalue_playercontroller) (break `GameplayAbilityActorInfo` (`self.GetActorInfo`)))
  (`/Engine/EditorBlueprintResources/StandardMacros.IsValid` _returnvalue_playercontroller
    (:`Is Valid`
      (`Controller.SetControlRotation` _returnvalue_playercontroller NewRotation))
    (:`Is Not Valid`
      (`Actor.K2_SetActorRotation` _returnvalue_owneractor NewRotation true))))

(event `AttackTarget`)

(event `self.MontageFinished`
  (params (`Finish Notify Index` :type Integer))
  (`/Engine/EditorBlueprintResources/StandardMacros.IncrementInt` (`self.TargetIndex`)
    (:`  `
      (`self.AttackNextTarget`))))

(event `WaitForTargetHit`
  (bind (_asynctaskproxy _payload) (`AbilityAsync_WaitGameplayEvent.WaitGameplayEventToActor` (`self.GetOwningActorFromActorInfo`) (struct :`TagName` "Event.TargetHit"))
    (:`EventReceived`
      (bind _asactor (cast `Actor` (`.OptionalObject` (break `GameplayEventData` _payload))))
      (`self.TargetHit` _asactor))))

(event `TargetHit`
  (params (Actor :type "Actor Object Reference"))
  (`self.ChangeAttributeOnActorByAmount` (`self.Damage Type`) (`self.Damage`) Actor))

(event `self.K2_OnEndAbility`
  (params (bWasCancelled :type Boolean))
  (`parent.K2_OnEndAbility` bWasCancelled))