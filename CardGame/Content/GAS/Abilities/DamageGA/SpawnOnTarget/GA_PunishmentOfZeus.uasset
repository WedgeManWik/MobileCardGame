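; GA_PunishmentOfZeus is a card-based gameplay ability that strikes a single selected target with lightning.
; On activation it requests one target, then spends the card's mana and plays a montage.
; The montage notify focuses on the target, spawns an unattached lightning particle effect on it and applies damage through a gameplay effect.
; The particle component is destroyed after a short delay.
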(event `self.K2_ActivateAbility`
  (`parent.K2_ActivateAbility`)
  (`self.SelectTargets` 1))

(event `self.TargetsHaveBeenSelected`
  (bind _targets (message `/Game/Cards/BI_CardUser.GetSelectedTargets` (`self.GetOwningActorFromActorInfo`)))
  (set `self.Target` (`|GetArrayItem` _targets))
  (`self.StartAttack`))

(event `self.StartAttack`
  (`self.UseCardMana`)
  (`self.PlayMontageAndWaitForNotify` "NewEnumerator3"))

(event `self.MontageNotify`
  (params (NotifyIndex :type Integer))
  (`self.AttackTarget`))

(event `self.AttackTarget`
  (bind _target (`self.Target`))
  (`self.FocusOnTarget`)
  (bind _particleref (`self.SpawnParticleEffectsOnActor` _target "/Game/VFX/FXVarietyPack/Particles/P_ky_lightning3.P_ky_lightning3"))
  (`self.ChangeAttributeOnActorByAmount` (`self.Damage Type`) (`self.Damage`) _target)
  (`KismetSystemLibrary.Delay` 1.0)
  (`ActorComponent.K2_DestroyComponent` _particleref))