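; Gameplay ability for a poison gas card that deals magic damage over time to selected targets.
; Activation runs target selection, then plays a montage whose notify pays the card cost and plays an impact sound.
; Each target gets a BC_ApplyGEOverTime component applying GE_MagicDamage periodically, plus a poison aura particle on the floor.
; Spawned particles are tracked and destroyed after a delay once the montage finishes, then the ability ends.
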(event `self.K2_ActivateAbility`
  (`parent.K2_ActivateAbility`)
  (`self.SelectTargets` 2))

(event `self.TargetsHaveBeenSelected`
  (`self.PlayMontageAndWaitForNotify` "NewEnumerator2"))

(event `self.MontageNotify`
  (params (NotifyIndex :type Integer))
  (`self.UseCardCost`)
  (`GameplayStatics.PlaySound2D` "/Game/Audio/AbilitySFX/SpecificDownloads/407992-Elemental_-Poison_Impact-1.407992-Elemental_-Poison_Impact-1" 1.0 1.0 0.0 null null)
  (bind _targets (message `/Game/Cards/BI_CardUser.GetSelectedTargets` (`self.GetOwningActorFromActorInfo`)))
  (for _array_element _targets
    (`|AddComponentByClass` _array_element "/Game/Components/BC_ApplyGEOverTime.BC_ApplyGEOverTime_C" (`self.Damage`) 4.0 0.25 "/Game/GAS/Effects/GE_MagicDamage.GE_MagicDamage_C" (`self.GetOwningActorFromActorInfo`))
    (bind _particleref (`self.SpawnParticleEffectsOnActor` _array_element "/Game/VFX/InfinityBladeEffects/Effects/FX_Skill_Aura/P_AuraCircle_Poison_Base_01.P_AuraCircle_Poison_Base_01" false true))
    (`KismetArrayLibrary.Array_Add` (`self.ParticlesSpawned`) _particleref)))

(event `self.MontageFinished`
  (params (`Finish Notify Index` :type Integer))
  (`KismetSystemLibrary.Delay` 2.0)
  (for _array_element (`self.ParticlesSpawned`)
    (`ActorComponent.K2_DestroyComponent` _array_element))
  (`KismetSystemLibrary.Delay` 1.0)
  (`self.FinishAbility`))