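; Card-based chain lightning gameplay ability that spends the card cost and attacks every enemy in sequence.
; On activation it sets all enemies as the selected targets, then starts the inherited attack loop.
; For each target it focuses and plays a montage, whose notify spawns a short-lived lightning emitter on the target and applies damage through a gameplay effect.
; When the montage finishes, it pauses briefly, then advances to the next target.
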(event `self.K2_ActivateAbility`
  (bind _returnvalue (`self.GetOwningActorFromActorInfo`))
  (`parent.K2_ActivateAbility`)
  (`self.UseCardCost`)
  (bind _enemies (message `/Game/Cards/BI_CardUser.GetAllEnemies` _returnvalue))
  (message `/Game/Cards/BI_CardUser.SetSelectedTargets` _returnvalue _enemies)
  (`self.StartAttack`))

(event `self.AttackTarget`
  (`self.FocusOnTarget`)
  (`self.PlayMontageAndWaitForNotify` "NewEnumerator1"))

(event `self.MontageNotify`
  (params (NotifyIndex :type Integer))
  (bind _target (`self.Target`))
  (bind _particleref (`self.SpawnParticleEffectsOnActor` _target "/Game/VFX/FXVarietyPack/Particles/P_ky_lightning3.P_ky_lightning3"))
  (`self.ChangeAttributeOnActorByAmount` (`self.Damage Type`) (`self.Damage`) _target)
  (`KismetSystemLibrary.Delay` 1.0)
  (`ActorComponent.K2_DestroyComponent` _particleref))

(event `self.MontageFinished`
  (params (`Finish Notify Index` :type Integer))
  (`KismetSystemLibrary.Delay` 0.2)
  (`/Engine/EditorBlueprintResources/StandardMacros.IncrementInt` (`self.TargetIndex`)
    (:`  `
      (`self.AttackNextTarget`))))