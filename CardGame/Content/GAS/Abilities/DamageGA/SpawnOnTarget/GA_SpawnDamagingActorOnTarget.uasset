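; Damage gameplay ability that spawns a configurable damaging actor directly at the location of its target.
; Activation defers to the parent, and the AttackTarget event focuses on the target before calling SpawnDamagingActorOnActor.
; That function uses the passed actor if valid, otherwise Target, and spawns ActorToSpawn owned by the ability's owning actor.
; The spawned actor receives its victim through a SetTargetToHit interface message.
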(event `self.K2_ActivateAbility`
  (`parent.K2_ActivateAbility`))

(event `self.AttackTarget`
  (`self.FocusOnTarget`)
  (`self.SpawnDamagingActorOnActor` null))

(fn `SpawnDamagingActorOnActor`
  (params (Actor :type "Actor Object Reference"))
  (locals (TargetActor :type Boolean))
  (bind _returnvalue (select `bool` (`KismetSystemLibrary.IsValid` Actor) :`false` (`self.Target`) :`true` Actor))
  (bind _returnvalue_2 (`|SpawnActorFromClass` (`self.ActorToSpawn`) (`KismetMathLibrary.MakeTransform` (`Actor.K2_GetActorLocation` _returnvalue)) "Undefined" "MultiplyWithRoot" (`self.GetOwningActorFromActorInfo`) null))
  (message `/Game/GAS/Abilities/AbilityActors/BI_AbilityActor.SetTargetToHit` _returnvalue_2 _returnvalue))