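; Gameplay ability for a melee attack that leaps at one selected target, deals physical damage and jumps back.
; After target selection, a montage notify stores the start location, attaches a spawned weapon mesh to a socket and starts the attack montage.
; Timed delays sequence two root-motion jump force tasks, toward the target and back, with damage applied on landing.
; The parent class supplies targeting and damage helpers; ending the ability destroys the weapon.
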(event `self.K2_ActivateAbility`
  (`parent.K2_ActivateAbility`)
  (`self.SelectTargets` 1))

(event `self.StartAttack`
  (bind _startlocation (`self.StartLocation`))
  (bind _returnvalue (`Actor.K2_GetActorLocation` (`self.Target`)))
  (bind _returnvalue_2 (`Actor.K2_GetActorLocation` (`self.GetAvatarActorFromActorInfo`)))
  (bind _returnvalue_3 (`Actor.K2_GetActorLocation` (`self.GetAvatarActorFromActorInfo`)))
  (message `/Game/Cards/BI_CardUser.PlayMontage` (`self.GetOwningActorFromActorInfo`) "NewEnumerator6")
  (`AbilityTask_WaitDelay.WaitDelay` 0.75
    (:`OnFinish`
      (bind _asynctaskproxy (`AbilityTask_ApplyRootMotionJumpForce.ApplyRootMotionJumpForce` "None" (`KismetMathLibrary.FindLookAtRotation` _returnvalue_2 _returnvalue) (- (`KismetMathLibrary.Vector_Distance` _returnvalue_2 _returnvalue) 100.0) 100.0 1.0 0.0 true "MaintainLastRootMotionVelocity")
        (:`then`
          (set `self.JumpTask` _asynctaskproxy))
        (:`OnFinish`
          (`GameplayTask.EndTask` (`self.JumpTask`))
          (bind _asynctaskproxy_2 (`AbilityTask_WaitDelay.WaitDelay` 0.2)
            (:`then`
              (set `self.WaitTask` _asynctaskproxy_2)
              (`self.DamageActor` (`self.Target`) "/Game/GAS/Effects/GE_PhysicalDamage.GE_PhysicalDamage_C"))
            (:`OnFinish`
              (`GameplayTask.EndTask` (`self.WaitTask`))
              (bind _asynctaskproxy_3 (`AbilityTask_ApplyRootMotionJumpForce.ApplyRootMotionJumpForce` "None" (`KismetMathLibrary.FindLookAtRotation` _returnvalue_3 _startlocation) (`KismetMathLibrary.Vector_Distance` _returnvalue_3 _startlocation) 100.0 1.0 0.0 true "MaintainLastRootMotionVelocity")
                (:`then`
                  (set `self.JumpTask` _asynctaskproxy_3))
                (:`OnFinish`
                  (`GameplayTask.EndTask` (`self.JumpTask`))
                  (`self.FinishAbility`))))))))))

(event `self.TargetsHaveBeenSelected`
  (bind _targets (message `/Game/Cards/BI_CardUser.GetSelectedTargets` (`self.GetOwningActorFromActorInfo`)))
  (set `self.Target` (`|GetArrayItem` _targets))
  (`self.PlayMontageAndWaitForNotify` "NewEnumerator7"))

(event `self.MontageNotify`
  (set `self.StartLocation` (`Actor.K2_GetActorLocation` (`self.GetOwningActorFromActorInfo`)))
  (`self.StopCurrentMontage`)
  (`self.SpawnWeaponInHand`)
  (`self.StartAttack`))

(event `SpawnWeaponInHand`
  (bind _returnvalue (`|SpawnActorFromClass` "/Script/Engine.SkeletalMeshActor" (`KismetMathLibrary.MakeTransform` (0.0 0.0 0.0)) "Undefined" "MultiplyWithRoot" (`self.GetOwningActorFromActorInfo`) null))
  (bind _output_get (set `self.SpawnedWeapon` _returnvalue))
  (`SkeletalMeshComponent.SetSkeletalMeshAsset` (`SkeletalMeshActor.SkeletalMeshComponent` _output_get) (`self.WeaponMesh`))
  (bind (_location _name) (message `/Game/Cards/BI_CardUser.GetSocketInfo` (`self.GetOwningActorFromActorInfo`) "NewEnumerator4"))
  (`SceneComponent.K2_AttachToComponent` (`SkeletalMeshActor.SkeletalMeshComponent` (`self.SpawnedWeapon`)) (`self.GetOwningComponentFromActorInfo`) _name "KeepRelative" "KeepRelative" "KeepRelative" true))

(event `self.K2_OnEndAbility`
  (params (bWasCancelled :type Boolean))
  (`parent.K2_OnEndAbility` bWasCancelled)
  (`Actor.K2_DestroyActor` (`self.SpawnedWeapon`)))