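; Base-style melee attack Gameplay Ability that handles target storage and a temporary weapon mesh.
; When targets are selected, it stores the first one and calls EquipWeapon, an empty hook here.
; SpawnWeaponInHand spawns a skeletal mesh actor and attaches it to a socket resolved through an owner message call.
; Ending the ability destroys the weapon and ends any valid jump or wait tasks.
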(event `self.K2_ActivateAbility`
  (`parent.K2_ActivateAbility`))

(event `self.TargetsHaveBeenSelected`
  (bind _targets (message `/Game/Cards/BI_CardUser.GetSelectedTargets` (`self.GetOwningActorFromActorInfo`)))
  (set `self.Target` (`|GetArrayItem` _targets))
  (`self.EquipWeapon`))

(event `EquipWeapon`)

(event `SpawnWeaponInHand`
  (bind _returnvalue (`|SpawnActorFromClass` "/Script/Engine.SkeletalMeshActor" (`KismetMathLibrary.MakeTransform` (0.0 0.0 0.0)) "Undefined" "MultiplyWithRoot" (`self.GetOwningActorFromActorInfo`) null))
  (bind _output_get (set `self.SpawnedWeapon` _returnvalue))
  (`SkeletalMeshComponent.SetSkeletalMeshAsset` (`SkeletalMeshActor.SkeletalMeshComponent` _output_get) (`self.WeaponMesh`))
  (bind (_location _name) (message `/Game/Cards/BI_CardUser.GetSocketInfo` (`self.GetOwningActorFromActorInfo`) (`self.SocketAttachWeapon`)))
  (`SceneComponent.K2_AttachToComponent` (`SkeletalMeshActor.SkeletalMeshComponent` (`self.SpawnedWeapon`)) (`self.GetOwningComponentFromActorInfo`) _name "KeepRelative" "KeepRelative" "KeepRelative" true))

(event `self.K2_OnEndAbility`
  (params (bWasCancelled :type Boolean))
  (bind _spawnedweapon (`self.SpawnedWeapon`))
  (bind _jumptask (`self.JumpTask`))
  (bind _waittask (`self.WaitTask`))
  (`parent.K2_OnEndAbility` bWasCancelled)
  (`/Engine/EditorBlueprintResources/StandardMacros.IsValid` _spawnedweapon
    (:`Is Valid`
      (`Actor.K2_DestroyActor` _spawnedweapon))
    (:`Is Not Valid`
      _))
  (`/Engine/EditorBlueprintResources/StandardMacros.IsValid` _jumptask
    (:`Is Valid`
      (`GameplayTask.EndTask` _jumptask))
    (:`Is Not Valid`
      _))
  (`/Engine/EditorBlueprintResources/StandardMacros.IsValid` _waittask
    (:`Is Valid`
      (`GameplayTask.EndTask` _waittask))))