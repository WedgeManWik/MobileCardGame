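; GA_ShatteringBlow is a card-cost melee ability that leaps at a single selected target, strikes it, then leaps back.
; Once the target is selected, it stores the start transform, pays the card cost and plays a montage whose notifies drive the sequence.
; The first notify launches a root-motion jump to just short of the target.
; The second applies damage and impact effects, then jumps back after a short delay, finishing the ability when that jump ends.
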(event `self.K2_ActivateAbility`
  (`parent.K2_ActivateAbility`)
  (`self.SelectTargets` 1))

(event `self.TargetsHaveBeenSelected`
  (`parent.TargetsHaveBeenSelected`)
  (set `self.StartTransform` (`Actor.GetTransform` (`self.GetAvatarActorFromActorInfo`)))
  (`self.UseCardCost`)
  (`self.PlayMontageAndWaitForNotify` "NewEnumerator17"))

(event `self.MontageNotify`
  (params (NotifyIndex :type Integer))
  (bind _starttransform_location (`KismetMathLibrary.BreakTransform` (`self.StartTransform`)))
  (bind _returnvalue (`Actor.K2_GetActorLocation` (`self.Target`)))
  (bind _returnvalue_2 (`Actor.K2_GetActorLocation` (`self.GetOwningActorFromActorInfo`)))
  (bind _returnvalue_3 (`Actor.K2_GetActorLocation` (`self.GetAvatarActorFromActorInfo`)))
  (switch `int` NotifyIndex
    (:`0`
      (`GameplayStatics.PlaySound2D` "/Game/Audio/AbilitySFX/Bundle1/AMP_Wind_Cast_02.AMP_Wind_Cast_02" 1.0 1.0 0.0 null null)
      (`AbilityTask_ApplyRootMotionJumpForce.ApplyRootMotionJumpForce` "None" (`KismetMathLibrary.FindLookAtRotation` _returnvalue_2 _returnvalue) (- (`KismetMathLibrary.Vector_Distance` _returnvalue_2 _returnvalue) 250.0) 100.0 0.65 0.0 true "MaintainLastRootMotionVelocity"))
    (:`1`
      (`self.SpawnParticleEffectsOnActor` (`self.Target`) "/Game/VFX/InfinityBladeEffects/Effects/FX_Mobile/Fire/combat/P_JumpAndDive_Fire_02.P_JumpAndDive_Fire_02" false true)
      (`self.ChangeAttributeOnActorByAmount` (`self.Damage Type`) (`self.Damage`) (`self.Target`))
      (`GameplayStatics.PlaySound2D` "/Game/Audio/AbilitySFX/Bundle1/AMP_Earth_Impact_01.AMP_Earth_Impact_01" 1.0 1.0 0.0 null null)
      (`KismetSystemLibrary.Delay` 0.5)
      (bind _asynctaskproxy (`AbilityTask_ApplyRootMotionJumpForce.ApplyRootMotionJumpForce` "None" (`KismetMathLibrary.FindLookAtRotation` _returnvalue_3 _starttransform_location) (`KismetMathLibrary.Vector_Distance` _returnvalue_3 _starttransform_location) 100.0 1.0 0.0 true "MaintainLastRootMotionVelocity")
        (:`then`
          (set `self.JumpTask` _asynctaskproxy)
          (message `/Game/Cards/BI_CardUser.PlayMontage` (`self.GetOwningActorFromActorInfo`) "NewEnumerator9" 0.0))
        (:`OnFinish`
          (`GameplayTask.EndTask` (`self.JumpTask`))
          (`self.FinishAbility`))))))