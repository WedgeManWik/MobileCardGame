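; Crippling Strike melee Gameplay Ability that dashes to a single selected target, damages it, then leaps back to where the attack began.
; Montage notifies sequence it: store the start transform, spawn the weapon and start the attack, dash to just short of the target, then apply damage through a gameplay effect.
; When the montage finishes, a root-motion jump returns the avatar to the stored position and ends the ability.
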(event `self.K2_ActivateAbility`
  (`parent.K2_ActivateAbility`)
  (`self.SelectTargets` 1))

(event `self.EquipWeapon`
  (`self.PlayMontageAndWaitForNotify` "NewEnumerator7"))

(event `self.MontageNotify`
  (params (NotifyIndex :type Integer))
  (switch `int` NotifyIndex
    (:`0`
      (set `self.StartTransform` (`Actor.GetTransform` (`self.GetOwningActorFromActorInfo`)))
      (`self.StopCurrentMontage`)
      (`self.SpawnWeaponInHand`)
      (`self.StartAttack`))
    (:`1`
      (`self.Dash`))
    (:`2`
      (`self.ChangeAttributeOnActorByAmount` (`self.Damage Type`) (`self.Damage`) (`self.Target`)))))

(event `self.MontageFinished`
  (params (`Finish Notify Index` :type Integer))
  (bind _starttransform_location (`KismetMathLibrary.BreakTransform` (`self.StartTransform`)))
  (bind _returnvalue (`Actor.K2_GetActorLocation` (`self.GetAvatarActorFromActorInfo`)))
  (switch `int` `Finish Notify Index`
    (:`0`
      (`AbilityTask_ApplyRootMotionJumpForce.ApplyRootMotionJumpForce` "None" (`KismetMathLibrary.FindLookAtRotation` _returnvalue _starttransform_location) (`KismetMathLibrary.Vector_Distance` _returnvalue _starttransform_location) 100.0 1.0 0.0 true "MaintainLastRootMotionVelocity"
        (:`then`
          (message `/Game/Cards/BI_CardUser.PlayMontage` (`self.GetOwningActorFromActorInfo`) "NewEnumerator9" 1.0))
        (:`OnFinish`
          (`KismetSystemLibrary.Delay` 0.2 :!label _label)
          (`self.StopCurrentMontage`)
          (`self.FinishAbility`))
        (:`OnLanded`
          (goto _label))))))

(event `self.StartAttack`
  (`parent.StartAttack`)
  (`self.PlayMontageAndWaitForNotify` "NewEnumerator13"))

(event `Dash`
  (bind _returnvalue (`Actor.K2_GetActorLocation` (`self.Target`)))
  (bind _returnvalue_2 (`Actor.K2_GetActorLocation` (`self.GetAvatarActorFromActorInfo`)))
  (`AbilityTask_ApplyRootMotionJumpForce.ApplyRootMotionJumpForce` "None" (`KismetMathLibrary.FindLookAtRotation` _returnvalue_2 _returnvalue) (- (`KismetMathLibrary.Vector_Distance` _returnvalue_2 _returnvalue) 150.0) 20.0 0.25 0.0 true "MaintainLastRootMotionVelocity"
    (:`OnFinish`
      (`self.PlayMontageAndWaitForNotify` "NewEnumerator14"))))