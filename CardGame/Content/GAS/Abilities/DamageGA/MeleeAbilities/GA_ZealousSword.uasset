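; GAS melee ability Zealous Sword: the character leaps at a single target, strikes it with a sword and leaps back.
; Parent-class target selection and weapon equip lead to a montage notify that stores the start transform, spawns the weapon and starts the attack.
; Chained delays and root motion jump-force tasks carry the attacker just short of the target, apply damage through a gameplay effect, then return it to the saved position and finish.
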(event `self.K2_ActivateAbility`
  (`parent.K2_ActivateAbility`)
  (`self.SelectTargets` 1))

(event `self.EquipWeapon`
  (`self.PlayMontageAndWaitForNotify` "NewEnumerator7"))

(event `self.MontageNotify`
  (params (NotifyIndex :type Integer))
  (switch `int` NotifyIndex
    (:`0`
      (set `self.StartTransform` (`Actor.GetTransform` (`self.GetOwningActorFromActorInfo`)))
      (`self.StopCurrentMontage`)
      (`self.SpawnWeaponInHand`)
      (`self.StartAttack`))))

(event `self.StartAttack`
  (bind _starttransform_location (`KismetMathLibrary.BreakTransform` (`self.StartTransform`)))
  (bind _returnvalue (`Actor.K2_GetActorLocation` (`self.Target`)))
  (bind _returnvalue_2 (`Actor.K2_GetActorLocation` (`self.GetAvatarActorFromActorInfo`)))
  (bind _returnvalue_3 (`Actor.K2_GetActorLocation` (`self.GetAvatarActorFromActorInfo`)))
  (`parent.StartAttack`)
  (message `/Game/Cards/BI_CardUser.PlayMontage` (`self.GetOwningActorFromActorInfo`) "NewEnumerator6" 1.0)
  (`AbilityTask_WaitDelay.WaitDelay` 0.75
    (:`OnFinish`
      (`AbilityTask_ApplyRootMotionJumpForce.ApplyRootMotionJumpForce` "None" (`KismetMathLibrary.FindLookAtRotation` _returnvalue_2 _returnvalue) (- (`KismetMathLibrary.Vector_Distance` _returnvalue_2 _returnvalue) 150.0) 100.0 0.65 0.0 true "SetVelocity"
        (:`OnFinish`
          (`AbilityTask_WaitDelay.WaitDelay` 0.2
            (:`then`
              (`self.ChangeAttributeOnActorByAmount` (`self.Damage Type`) (`self.Damage`) (`self.Target`)))
            (:`OnFinish`
              (`AbilityTask_WaitDelay.WaitDelay` 0.5
                (:`OnFinish`
                  (`AbilityTask_ApplyRootMotionJumpForce.ApplyRootMotionJumpForce` "None" (`KismetMathLibrary.FindLookAtRotation` _returnvalue_3 _starttransform_location) (`KismetMathLibrary.Vector_Distance` _returnvalue_3 _starttransform_location) 100.0 1.0 0.0 true "MaintainLastRootMotionVelocity"
                    (:`then`
                      (message `/Game/Cards/BI_CardUser.PlayMontage` (`self.GetOwningActorFromActorInfo`) "NewEnumerator9" 1.0))
                    (:`OnFinish`
                      (`self.FinishAbility`))))))))))))