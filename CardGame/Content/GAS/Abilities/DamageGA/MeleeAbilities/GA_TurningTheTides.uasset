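; Melee card ability Turning the Tides, a GAS ability that targets every enemy with a ground-burst and lightning display.
; Activation plays a montage whose first notify spawns the weapon in hand.
; The second pays the card cost, spawns a burst under the owner, then after a short delay sets all enemies as selected targets and spawns effects on each.
; After another delay it calls FinishAbility, with no damage applied in this graph.
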(event `self.K2_ActivateAbility`
  (`parent.K2_ActivateAbility`)
  (`self.PlayMontageAndWaitForNotify` "NewEnumerator7"))

(event `self.MontageNotify`
  (params (NotifyIndex :type Integer))
  (bind _returnvalue (`self.GetOwningActorFromActorInfo`))
  (switch `int` NotifyIndex
    (:`0`
      (`self.SpawnWeaponInHand`))
    (:`1`
      (`self.UseCardCost`)
      (`self.SpawnParticleEffectsOnActor` _returnvalue "/Game/VFX/InfinityBladeEffects/Effects/FX_Mobile/combat/P_JumpAndDive_Untyped_00.P_JumpAndDive_Untyped_00" false true)
      (`KismetSystemLibrary.Delay` 0.5)
      (bind _enemies (message `/Game/Cards/BI_CardUser.GetAllEnemies` _returnvalue))
      (message `/Game/Cards/BI_CardUser.SetSelectedTargets` _returnvalue _enemies)
      (for _array_element _enemies
        (`self.SpawnParticleEffectsOnActor` _array_element "/Game/VFX/InfinityBladeEffects/Effects/FX_Mobile/combat/P_JumpAndDive_Untyped_00.P_JumpAndDive_Untyped_00" false true)
        (`self.SpawnParticleEffectsOnActor` _array_element "/Game/VFX/FXVarietyPack/Particles/P_ky_lightning1.P_ky_lightning1" false true))
      (`KismetSystemLibrary.Delay` 1.0)
      (`self.FinishAbility`))))