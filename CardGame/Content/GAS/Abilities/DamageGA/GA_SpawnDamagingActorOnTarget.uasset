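; Gameplay ability that attacks a target by spawning a damaging actor on it.
; Activation defers to the parent ability, and the AttackTarget event calls SpawnDamagingActorOnActor.
; That function spawns the ActorToSpawn class at the Target's location, owned by the ability's owning actor, then passes it the Target through a SetTargetToHit message.
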(event `self.K2_ActivateAbility`
  (`parent.K2_ActivateAbility`))

(event `self.AttackTarget`
  (`self.SpawnDamagingActorOnActor`))

(fn `SpawnDamagingActorOnActor`
  (bind _target (`self.Target`))
  (bind _returnvalue (`|SpawnActorFromClass` (`self.ActorToSpawn`) (`KismetMathLibrary.MakeTransform` (`Actor.K2_GetActorLocation` _target)) "Undefined" "MultiplyWithRoot" (`self.GetOwningActorFromActorInfo`) null))
  (message `/Game/GAS/Abilities/AbilityActors/BI_AbilityActor.SetTargetToHit` _returnvalue _target))