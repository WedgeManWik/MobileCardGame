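; Gameplay ability that spends a card cost and launches a damaging projectile at a selected target.
; Target selection starts the attack, the owner focuses on the target, and a montage notify reads the launch socket's location.
; It spawns the projectile class there facing the target and passes it that target, ending the ability if none is valid.
; A projectile miss is relayed to the owner as a missed-target gameplay event.
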(event `self.K2_ActivateAbility`
  (`parent.K2_ActivateAbility`))

(event `self.TargetsHaveBeenSelected`
  (`self.StartAttack`))

(event `self.StartAttack`
  (`self.UseCardCost`)
  (`parent.StartAttack`))

(event `self.AttackTarget`
  (`parent.AttackTarget`)
  (`self.FocusOnTarget`))

(event `self.MontageNotify`
  (params (NotifyIndex :type Integer))
  (bind _location (message `/Game/Cards/BI_CardUser.GetSocketInfo` (`self.GetOwningActorFromActorInfo`) (`self.SocketToLaunchProjectileFrom`)))
  (set `self.SpawnLocation` _location)
  (`self.Launch Damaging Projectile at Target` null))

(event `self.K2_OnEndAbility`
  (params (bWasCancelled :type Boolean))
  (`parent.K2_OnEndAbility` bWasCancelled))

(fn `Launch Damaging Projectile at Target`
  (params (Target :type "Actor Object Reference"))
  (returns (Projectile :type "Actor Object Reference"))
  (locals (AffectedTarget :type "Actor Object Reference"))
  (bind _spawnlocation (`self.SpawnLocation`))
  (bind _target (`self.Target`))
  (`/Engine/EditorBlueprintResources/StandardMacros.IsValid` Target
    (:`Is Valid`
      (set `local.AffectedTarget` Target)
      (bind _returnvalue (`|SpawnActorFromClass` (`self.ProjectileClass`) (`KismetMathLibrary.MakeTransform` _spawnlocation (`KismetMathLibrary.FindLookAtRotation` _spawnlocation (`Actor.K2_GetActorLocation` (`local.AffectedTarget`)))) "Undefined" "MultiplyWithRoot" (`self.GetOwningActorFromActorInfo`) null :!label _label))
      (message `/Game/GAS/Abilities/AbilityActors/BI_AbilityActor.SetTargetToHit` _returnvalue (`local.AffectedTarget`))
      (add `/Game/GAS/Abilities/AbilityActors/BP_AbilityActor.MissedTarget` _returnvalue (`|CreateDelegate` :!event `Projectile Missed Target`))
      (return _returnvalue))
    (:`Is Not Valid`
      (`/Engine/EditorBlueprintResources/StandardMacros.IsValid` _target
        (:`Is Valid`
          (set `local.AffectedTarget` _target)
          (goto _label))
        (:`Is Not Valid`
          (`self.K2_EndAbility`))))))

(fn `Projectile Missed Target`
  (`AbilitySystemBlueprintLibrary.SendGameplayEventToActor` (`self.GetOwningActorFromActorInfo`) (struct :`TagName` "Event.MissedTarget")))