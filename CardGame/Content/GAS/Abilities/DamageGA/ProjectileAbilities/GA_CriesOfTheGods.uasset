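; GA_CriesOfTheGods is a card-driven Gameplay Ability that rains damaging projectiles on every enemy.
; Projectile count and damage come from card data by ability level and upgrade state.
; On the montage notify, it launches projectiles from random points above each enemy, spawning higher for each successive one.
; A hit-or-miss countdown finishes the ability, with a timed delay also calling finish.
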(event `self.InitialiseCardStats`
  (bind (_gameplayability _description _normalamounts _upgradedamounts _downgradedamounts) (break `/Game/Cards/S_GA_Details` (`|GetArrayItem` (`.Abilities_78_195985E04BEB039D5D89D0BF920AEA2F` (break `/Game/Cards/S_CardInfo` (`self.CardInfo`))) (`self.GetAbilityLevel`))))
  (bind _returnvalue (select `/Game/Cards/E_CardUpgradedState` (`self.Upgrade State`) :`NewEnumerator0` _normalamounts :`NewEnumerator1` _upgradedamounts :`NewEnumerator2` _downgradedamounts))
  (bind _output_amount (break `/Game/Cards/S_AmountType` (`|GetArrayItem` _returnvalue)))
  (bind _output_amount_2 (break `/Game/Cards/S_AmountType` (`|GetArrayItem` _returnvalue 1)))
  (set `self.NumProjectilesToSpawn` (`KismetMathLibrary.FTrunc` _output_amount))
  (set `self.Damage` _output_amount_2))

(event `self.K2_ActivateAbility`
  (`parent.K2_ActivateAbility`)
  (`self.WaitForTargetHit`)
  (`self.PlayMontageAndWaitForNotify` "NewEnumerator0")
  (`self.UseCardCost`))

(event `self.MontageNotify`
  (params (NotifyIndex :type Integer))
  (bind _enemies (message `/Game/Cards/BI_CardUser.GetAllEnemies` (`self.GetOwningActorFromActorInfo`)))
  (set `self.NumHitsLeft` (* (`KismetArrayLibrary.Array_Length` _enemies) (`self.NumProjectilesToSpawn`)))
  (for (_array_element _array_index) _enemies
    (set `self.Target` _array_element)
    (for _ (range 1 (+ (`self.NumProjectilesToSpawn`) 1))
      (set `self.SpawnLocation` (`KismetMathLibrary.RandomPointInBoundingBox` (+ (`Actor.K2_GetActorLocation` (`self.Target`)) (`KismetMathLibrary.MakeVector` 0.0 0.0 (+ (* _array_index 500) 1000))) (500.0 500.0 500.0)))
      (`self.Launch Damaging Projectile at Target` null)))
  (`KismetSystemLibrary.Delay` 7.0)
  (`self.FinishAbility`))

(event `self.MontageFinished`
  (params (`Finish Notify Index` :type Integer)))

(event `self.TargetHit`
  (params (Actor :type "Actor Object Reference"))
  (`parent.TargetHit` Actor)
  (`self.RegisterHit`))

(event `RegisterHit`
  (bind _result (`/Engine/EditorBlueprintResources/StandardMacros.DecrementInt` (`self.NumHitsLeft`) :!label _label)
    (:`  `
      (if (== _result 0)
        (`self.FinishAbility`)))))

(event `self.MissedTarget`
  (goto _label))

(fn `Projectile Missed Target`
  (`parent.Projectile Missed Target`)
  (`self.RegisterHit`))