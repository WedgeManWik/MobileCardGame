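; Sorcery Shatter gameplay ability that fires damaging projectiles at up to two selected targets.
; After target selection it pays the card cost and plays a slowed montage.
; Each montage notify launches a projectile from alternating sockets, with the first pair aimed at the first target and the second pair at the second, or all at a lone target.
; The ability finishes shortly after the montage ends.
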(event `self.K2_ActivateAbility`
  (`parent.K2_ActivateAbility`)
  (`self.SelectTargets` 2))

(event `self.TargetsHaveBeenSelected`
  (`self.UseCardCost`)
  (`self.PlayMontageAndWaitForNotify` "NewEnumerator19" 0.5)
  (`self.WaitForTargetHit`)
  (bind _targets (message `/Game/Cards/BI_CardUser.GetSelectedTargets` (`self.GetOwningActorFromActorInfo`)))
  (set `self.Target` (`|GetArrayItem` _targets))
  (set `self.NumTargetsToHit` (`KismetArrayLibrary.Array_Length` _targets)))

(event `self.MontageNotify`
  (params (NotifyIndex :type Integer))
  (bind _location (message `/Game/Cards/BI_CardUser.GetSocketInfo` (`self.GetOwningActorFromActorInfo`) (select `int` NotifyIndex :`0` "NewEnumerator0" :`1` "NewEnumerator1" :`2` "NewEnumerator0" :`3` "NewEnumerator1" :!type "/Game/Animations/E_SocketType Enum")))
  (set `self.SpawnLocation` _location)
  (if (> (`self.NumTargetsToHit`) 1)
    (switch `int` NotifyIndex
      (:`0`
        (`self.Launch Damaging Projectile at Target` (`self.Target`) :!label _label))
      (:`1`
        (goto _label))
      (:`2`
        (bind _targets (message `/Game/Cards/BI_CardUser.GetSelectedTargets` (`self.GetOwningActorFromActorInfo`) :!label _label_2))
        (set `self.Target` (`|GetArrayItem` _targets 1))
        (`self.Launch Damaging Projectile at Target` null))
      (:`3`
        (goto _label_2)))
    (else
      (`self.Launch Damaging Projectile at Target` (`self.Target`)))))

(event `self.MontageFinished`
  (params (`Finish Notify Index` :type Integer))
  (`KismetSystemLibrary.Delay` 1.0)
  (`self.FinishAbility`))