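; Hatchet Hail is a projectile damage ability that attacks every enemy in sequence.
; On activation it sets all enemies as the owner's selected targets, then starts the parent attack flow.
; Each attack spawns an axe mesh on a socket and plays a sped-up montage.
; The montage notify destroys that axe before deferring to the parent, and montage completion advances to the next target after a short delay.
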(event `self.K2_ActivateAbility`
  (bind _returnvalue (`self.GetOwningActorFromActorInfo`))
  (`parent.K2_ActivateAbility`)
  (bind _enemies (message `/Game/Cards/BI_CardUser.GetAllEnemies` _returnvalue))
  (message `/Game/Cards/BI_CardUser.SetSelectedTargets` _returnvalue _enemies)
  (`self.StartAttack`))

(event `self.AttackTarget`
  (bind _actorref (`self.SpawnActorAttachedToSocket` "/Script/Engine.SkeletalMeshActor" "NewEnumerator4"))
  (bind _asskeletal_mesh_actor (cast `SkeletalMeshActor` _actorref))
  (`SkeletalMeshComponent.SetSkeletalMeshAsset` (`SkeletalMeshActor.SkeletalMeshComponent` _asskeletal_mesh_actor) "/Game/InfinityBladeWeapons/Weapons/Blade/Axes/Blade_DeadlyAxe/SK_Blade_DeadlyAxe.SK_Blade_DeadlyAxe")
  (set `self.SpawnedHatchet` _actorref)
  (`self.PlayMontageAndWaitForNotify` "NewEnumerator15" 2.0))

(event `self.MontageNotify`
  (params (NotifyIndex :type Integer))
  (`Actor.K2_DestroyActor` (`self.SpawnedHatchet`))
  (`parent.MontageNotify` NotifyIndex))

(event `self.MontageFinished`
  (params (`Finish Notify Index` :type Integer))
  (`KismetSystemLibrary.Delay` 0.2)
  (`/Engine/EditorBlueprintResources/StandardMacros.IncrementInt` (`self.TargetIndex`)
    (:`  `
      (`self.AttackNextTarget`))))