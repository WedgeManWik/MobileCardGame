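; Gameplay ability base or variant, named for projectiles launched at a target, that supplies a DamageTarget function for applying damage.
; DamageTarget builds a magic or physical damage effect spec based on IsMagicDamage and sets the absolute Damage as a SetByCaller magnitude under Event.Damage.
; The owner's ability system component applies that spec to the target.
; Its activation and end events are disabled stubs, so this graph contains no launch logic.
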(fn `DamageTarget`
  (params (Target :type "Actor Object Reference"))
  (locals (TargetToDamage :type "Actor Object Reference"))
  (bind _returnvalue (`self.GetAbilitySystemComponentFromActorInfo`))
  (`/Engine/EditorBlueprintResources/StandardMacros.IsValid` Target
    (:`Is Valid`
      (set `local.TargetToDamage` Target))
    (:`Is Not Valid`
      (set `local.TargetToDamage` (`self.Target`))))
  (bind _returnvalue_2 (`AbilitySystemBlueprintLibrary.AssignTagSetByCallerMagnitude` (`AbilitySystemComponent.MakeOutgoingSpec` :`self` _returnvalue :`GameplayEffectClass` (select `bool` (`self.IsMagicDamage`) :`false` "/Game/GAS/Effects/GE_PhysicalDamage.GE_PhysicalDamage_C" :`true` "/Game/GAS/Effects/GE_MagicDamage.GE_MagicDamage_C" :!type "GameplayEffect Class Reference")) (struct :`TagName` "Event.Damage") (`KismetMathLibrary.Abs` (`self.Damage`))))
  (`AbilitySystemComponent.BP_ApplyGameplayEffectSpecToTarget` _returnvalue _returnvalue_2 (`AbilitySystemBlueprintLibrary.GetAbilitySystemComponent` (`local.TargetToDamage`))))