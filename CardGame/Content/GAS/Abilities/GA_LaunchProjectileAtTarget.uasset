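; Gameplay ability that launches a projectile of a configurable class at a target actor.
; On activation it spawns the projectile at SpawnLocation, rotated toward the target and owned by the ability's owning actor.
; It passes the target to the projectile and binds to its missed-target callback.
; On a miss it sends the Event.TargetHit gameplay event to the owner, despite the tag's name.
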(event `self.K2_ActivateAbility`
  (bind _spawnlocation (`self.SpawnLocation`))
  (`parent.K2_ActivateAbility`)
  (bind _returnvalue (`|SpawnActorFromClass` (`self.ProjectileClass`) (`KismetMathLibrary.MakeTransform` _spawnlocation (`KismetMathLibrary.FindLookAtRotation` _spawnlocation (`Actor.K2_GetActorLocation` (`self.Target`)))) "Undefined" "MultiplyWithRoot" (`self.GetOwningActorFromActorInfo`) null))
  (message `/Game/GAS/Abilities/AbilityActors/BI_AbilityActor.SetTargetToHit` _returnvalue (`self.Target`))
  (add `/Game/GAS/Abilities/AbilityActors/BP_AbilityActor.MissedTarget` _returnvalue (delegate `MissedTarget`)))

(event `MissedTarget`
  (`AbilitySystemBlueprintLibrary.SendGameplayEventToActor` (`self.GetOwningActorFromActorInfo`) (struct :`TagName` "Event.TargetHit")))

(event `self.K2_OnEndAbility`
  (params (bWasCancelled :type Boolean))
  (`parent.K2_OnEndAbility` bWasCancelled))