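; Base Gameplay Ability for card actions, loading the used card's row from DT_Cards and providing hooks for child abilities.
; Target selection auto-picks a lone enemy or grants GA_SelectTargets and awaits an event.
; Helpers apply mana and energy costs, send attribute changes as event payloads, relay montage notifies through gameplay events, and spawn effects or attached actors.
; Finishing sends an event that ends the ability and restores the owner's starting transform.
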(event `SelectTargets`
  (params (NumMaxTargets :type Integer))
  (bind _returnvalue (`self.GetOwningActorFromActorInfo`))
  (bind _enemies (message `/Game/Cards/BI_CardUser.GetAllEnemies` _returnvalue))
  (if (and (== (`KismetArrayLibrary.Array_Length` _enemies) 1) (== NumMaxTargets 1))
    (message `/Game/Cards/BI_CardUser.SetSelectedTargets` _returnvalue _enemies)
    (`self.TargetsHaveBeenSelected`)
    (else
      (`AbilitySystemComponent.K2_GiveAbilityAndActivateOnce` (`self.GetAbilitySystemComponentFromActorInfo`) "/Game/GAS/Abilities/SelectTargets/GA_SelectTargets.GA_SelectTargets_C" NumMaxTargets -1)
      (`AbilityTask_WaitGameplayEvent.WaitGameplayEvent` (struct :`TagName` "Action.TargetsSet") null true
        (:`EventReceived`
          (`self.TargetsHaveBeenSelected`))))))

(event `self.K2_ActivateAbility`
  (`self.InitialiseAbility`))

(event `FinishAbility`
  (`AbilitySystemBlueprintLibrary.SendGameplayEventToActor` (`self.GetOwningActorFromActorInfo`) (struct :`TagName` "Event.Ability.Finished"))
  (`Actor.K2_SetActorTransform` (`self.GetOwningActorFromActorInfo`) (`self.StartTransform`) false true))

(event `InitialiseCardStats`)

(event `TargetsHaveBeenSelected`)

(event `Cancel Ability`
  (bind (_returnvalue_owneractor _returnvalue_avataractor _returnvalue_playercontroller) (break `GameplayAbilityActorInfo` (`self.GetActorInfo`)))
  (message `/Game/Cards/BI_CardUser.CancelCardBeingUsed` (select `bool` (`KismetSystemLibrary.IsValid` _returnvalue_playercontroller) :`false` _returnvalue_owneractor :`true` _returnvalue_playercontroller :!type "Object Object Reference"))
  (`self.FinishAbility`))

(event `InitialiseAbility`
  (set `self.StartTransform` (`Actor.GetTransform` (`self.GetOwningActorFromActorInfo`)))
  (`self.InitialiseCard`)
  (`AbilityAsync_WaitGameplayEvent.WaitGameplayEventToActor` (`self.GetOwningActorFromActorInfo`) (struct :`TagName` "Event.Ability.Finished")
    (:`EventReceived`
      (`self.K2_EndAbility`))))

(event `ChangeAttributeOnActorByAmount`
  (params (GameplayEffectClass :type "GameplayEffect Class Reference") (Amount :type "Float (single-precision)") (Actor :type "Actor Object Reference"))
  (bind _returnvalue (`self.GetOwningActorFromActorInfo`))
  (bind _returnvalue_2 (`|GenericCreateObject` "/Game/GAS/DataAssets/DA_ChangeAttribute.DA_ChangeAttribute_C" Amount _returnvalue GameplayEffectClass))
  (`AbilitySystemBlueprintLibrary.SendGameplayEventToActor` Actor (struct :`TagName` "Attribute.ChangeAmount") (make `GameplayEventData` (struct :`TagName` "Attribute.ChangeAmount") _returnvalue Actor _returnvalue_2)))

(event `PlayMontageAndWaitForNotify`
  (params (MontageToPlay :type "/Game/Animations/E_CharacterMontage Enum" :default "NewEnumerator0") (PlayRate :type "Float (double-precision)" :default 1.0))
  (bind _returnvalue (`self.GetOwningActorFromActorInfo`))
  (bind _finishnotifyindex (`self.FinishNotifyIndex`))
  (bind _notifyindex (`self.NotifyIndex`))
  (`self.StopCurrentMontage`)
  (bind _asynctaskproxy (`AbilityAsync_WaitGameplayEvent.WaitGameplayEventToActor` _returnvalue (struct :`TagName` "Event.MontageNotify"))
    (:`then`
      (set `self.WaitMontageNotify` _asynctaskproxy)
      (message `/Game/Cards/BI_CardUser.PlayMontage` _returnvalue MontageToPlay PlayRate)
      (bind _asynctaskproxy_2 (`AbilityAsync_WaitGameplayEvent.WaitGameplayEventToActor` _returnvalue (struct :`TagName` "Event.MontageFinished"))
        (:`then`
          (set `self.WaitMontageFinished` _asynctaskproxy_2))
        (:`EventReceived`
          (`self.MontageFinished` _finishnotifyindex)
          (`/Engine/EditorBlueprintResources/StandardMacros.IncrementInt` _finishnotifyindex
            (:`  `
              (`AbilityAsync.EndAction` (`self.WaitMontageFinished`)))))))
    (:`EventReceived`
      (`self.MontageNotify` _notifyindex)
      (`/Engine/EditorBlueprintResources/StandardMacros.IncrementInt` _notifyindex))))

(event `StopCurrentMontage`
  (bind _waitmontagenotify (`self.WaitMontageNotify`))
  (bind _waitmontagefinished (`self.WaitMontageFinished`))
  (`self.MontageStop` -1.0)
  (`/Engine/EditorBlueprintResources/StandardMacros.IsValid` _waitmontagenotify
    (:`Is Valid`
      (`AbilityAsync.EndAction` _waitmontagenotify))
    (:`Is Not Valid`
      _))
  (`/Engine/EditorBlueprintResources/StandardMacros.IsValid` _waitmontagefinished
    (:`Is Valid`
      (`AbilityAsync.EndAction` _waitmontagefinished))))

(event `MontageNotify`
  (params (NotifyIndex :type Integer)))

(event `MontageFinished`
  (params (`Finish Notify Index` :type Integer)))

(event `UseCardCost`
  (bind (_cardinfo_name _cardinfo_image _cardinfo_description _cardinfo_backgroundcolour _cardinfo_abilities _cardinfo_manacost _cardinfo_energycost) (break `/Game/Cards/S_CardInfo` (`self.CardInfo`)))
  (if (== (`self.GetAbilityLevel`) 0)
    (`KismetSystemLibrary.Delay` 0.05)
    (bind _result (`/Engine/EditorBlueprintResources/StandardMacros.NegateInt` _cardinfo_manacost)
      (:`  `
        (bind _returnvalue (`AbilitySystemBlueprintLibrary.AssignTagSetByCallerMagnitude` (`self.MakeOutgoingGameplayEffectSpec` "/Game/GAS/Effects/GE_ChangeManaBy.GE_ChangeManaBy_C") (struct :`TagName` "Attribute.ChangeAmount") (`KismetMathLibrary.Conv_IntToDouble` _result)))
        (`self.K2_ApplyGameplayEffectSpecToOwner` _returnvalue)
        (bind _result_2 (`/Engine/EditorBlueprintResources/StandardMacros.NegateInt` _cardinfo_energycost)
          (:`  `
            (bind _returnvalue_2 (`AbilitySystemBlueprintLibrary.AssignTagSetByCallerMagnitude` (`self.MakeOutgoingGameplayEffectSpec` "/Game/GAS/Effects/GE_ChangeEnergyBy.GE_ChangeEnergyBy_C") (struct :`TagName` "Attribute.ChangeAmount") (`KismetMathLibrary.Conv_IntToDouble` _result_2)))
            (`self.K2_ApplyGameplayEffectSpecToOwner` _returnvalue_2)))))))

(event `self.K2_OnEndAbility`
  (params (bWasCancelled :type Boolean)))

(fn `InitialiseCard`
  (bind _returnvalue (`self.GetOwningActorFromActorInfo`))
  (`/Engine/EditorBlueprintResources/StandardMacros.IsValid` _returnvalue
    (:`Is Valid`
      (bind (_cardid _widgetref _upgradestate) (message `/Game/Cards/BI_CardUser.GetCardBeingUsed` _returnvalue))
      (bind _returnvalue_2 (`|GetDataTableRow` "/Game/Cards/DT_Cards.DT_Cards" _cardid)
        (:`then`
          (set `self.CardInfo` _returnvalue_2)
          (set `self.Upgrade State` _upgradestate)
          (`self.InitialiseCardStats`))
        (:`RowNotFound`
          (`self.K2_EndAbility`))))
    (:`Is Not Valid`
      (`self.K2_EndAbility`))))

(fn `SpawnActorAttachedToSocket`
  (params (ActorClass :type "Actor Class Reference") (SocketType :type "/Game/Animations/E_SocketType Enum" :default "NewEnumerator0"))
  (returns (ActorRef :type "Actor Object Reference"))
  (bind _returnvalue (`|SpawnActorFromClass` ActorClass (`KismetMathLibrary.MakeTransform` (0.0 0.0 0.0)) "Undefined" "MultiplyWithRoot" (`self.GetOwningActorFromActorInfo`) null))
  (bind (_location _name) (message `/Game/Cards/BI_CardUser.GetSocketInfo` (`self.GetAvatarActorFromActorInfo`) SocketType))
  (`Actor.K2_AttachToComponent` _returnvalue (`self.GetOwningComponentFromActorInfo`) _name "SnapToTarget" "SnapToTarget" "SnapToTarget" true)
  (return _returnvalue))

(fn `SpawnParticleEffectsOnActor`
  (params (Actor :type "Actor Object Reference") (EmitterTemplate :type "ParticleSystem Object Reference") (AttachToActor :type Boolean) (OnFloor :type Boolean))
  (returns (ParticleRef :type "ParticleSystemComponent Object Reference"))
  (bind _location (message `/Game/Cards/BI_CardUser.GetSocketInfo` Actor "NewEnumerator5"))
  (bind _returnvalue (`GameplayStatics.SpawnEmitterAtLocation` EmitterTemplate (select `bool` OnFloor :`false` (`Actor.K2_GetActorLocation` Actor) :`true` _location)))
  (set `self.ParticleFX` _returnvalue)
  (if AttachToActor
    (`SceneComponent.K2_AttachToComponent` (`self.ParticleFX`) (`Actor.GetComponentByClass` Actor "/Script/Engine.SkeletalMeshComponent") "None" "SnapToTarget" "SnapToTarget" "KeepRelative" true))
  (return (`self.ParticleFX`)))