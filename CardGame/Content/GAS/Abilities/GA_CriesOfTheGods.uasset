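; Gameplay ability for the Cries of the Gods card, which launches fireballs from the owner at selected targets.
; It requests target selection, waits for Action.TargetsSet, then commits and applies the card's DT_Cards mana cost through a SetByCaller GE_UseMana.
; It spawns a BP_FireBall facing each target, passing every fireball the full target list.
; The ability ends on Event.TargetHit or a failed commit.
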(event `self.K2_ActivateAbility`
  (bind _returnvalue (`self.GetOwningActorFromActorInfo`))
  (bind _returnvalue_2 (`self.GetOwningActorFromActorInfo`))
  (bind _returnvalue_3 (`Actor.K2_GetActorLocation` _returnvalue))
  (`AbilityTask_WaitGameplayEvent.WaitGameplayEvent` (struct :`TagName` "Action.TargetsSet") null
    (:`then`
      (message `/Game/Cards/BI_CardUser.SelectTargetsToUseOnCard` _returnvalue_2 1))
    (:`EventReceived`
      (bind _returnvalue_4 (`self.K2_CommitAbility`))
      (if _returnvalue_4
        (bind _cardid (message `/Game/Cards/BI_CardUser.GetCardBeingUsed` _returnvalue_2))
        (bind _returnvalue_5 (`|GetDataTableRow` "/Game/Cards/DT_Cards.DT_Cards" _cardid)
          (:`then`
            (bind _returnvalue_6 (`AbilitySystemBlueprintLibrary.AssignTagSetByCallerMagnitude` (`self.MakeOutgoingGameplayEffectSpec` "/Game/GAS/Effects/GE_UseMana.GE_UseMana_C") (struct :`TagName` "Mana.UseCard") (`KismetMathLibrary.Conv_IntToDouble` (`.ManaCost_48_8FF30D184009C0298630518A94D8FAEA` (break `/Game/Cards/S_CardInfo` _returnvalue_5)))))
            (`self.K2_ApplyGameplayEffectSpecToOwner` _returnvalue_6)
            (bind _targets (message `/Game/Cards/BI_CardUser.GetSelectedTargets` _returnvalue))
            (for _array_element _targets
              (bind _returnvalue_7 (`|SpawnActorFromClass` "/Game/GAS/Abilities/AbilityActors/Projectiles/BP_FireBall.BP_FireBall_C" (`KismetMathLibrary.MakeTransform` _returnvalue_3 (`KismetMathLibrary.FindLookAtRotation` _returnvalue_3 (`Actor.K2_GetActorLocation` _array_element))) "Undefined" "MultiplyWithRoot" (`self.GetOwningActorFromActorInfo`) null))
              (`/Game/GAS/Abilities/AbilityActors/BP_AbilityActor.SetTargetsToHit` _returnvalue_7 _targets))
            (`AbilityTask_WaitGameplayEvent.WaitGameplayEvent` (struct :`TagName` "Event.TargetHit") null
              (:`EventReceived`
                (`self.K2_EndAbility`)))))
        (else
          (`self.K2_EndAbility`))))))