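; GA_ManaSurge is a card-driven gameplay ability that regenerates mana when an attribute value is a multiple of a threshold from the card's stats.
; On a match it plays a montage, whose notify calls RegenMana and spawns a particle effect; otherwise, after a delay, it cancels the card-in-use message.
; If the attribute also matches a second multiple, BC_ApplyGEOverTime grants bonus mana over time through GE_RegenerateMana.
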(event `self.InitialiseCardStats`
  (bind (_gameplayability _description _amounts) (break `/Game/Cards/S_GA_Details` (`|GetArrayItem` (`.Abilities_64_195985E04BEB039D5D89D0BF920AEA2F` (break `/Game/Cards/S_CardInfo` (`self.CardInfo`))))))
  (set `self.TotalManaGained` (`|GetArrayItem` _amounts))
  (set `self.FirstMultiple` (`|GetArrayItem` _amounts 1))
  (set `self.AdditionalManaGained` (`|GetArrayItem` _amounts 2))
  (set `self.SecondMultiple` (`|GetArrayItem` _amounts 3)))

(event `self.K2_ActivateAbility`
  (bind (_returnvalue_owneractor _returnvalue_avataractor _returnvalue_playercontroller) (break `GameplayAbilityActorInfo` (`self.GetActorInfo`)))
  (`parent.K2_ActivateAbility`)
  (if (== (mod (`.ReturnValue` (`AbilitySystemBlueprintLibrary.GetFloatAttributeFromAbilitySystemComponent` (`self.GetAbilitySystemComponentFromActorInfo`) (struct :`AttributeName` "Health" :`Attribute` "/Script/CardGame.GAAttributeSet:Health" :`AttributeOwner` "/Script/CoreUObject.Class'\"/Script/CardGame.GAAttributeSet\"'"))) (`self.FirstMultiple`)) 0.0)
    (`self.PlayMontageAndWaitForNotify` "NewEnumerator2")
    (else
      (`KismetSystemLibrary.Delay` 1.0)
      (`/Engine/EditorBlueprintResources/StandardMacros.IsValid` _returnvalue_playercontroller
        (:`Is Valid`
          (message `/Game/Cards/BI_CardUser.CancelCardBeingUsed` _returnvalue_playercontroller))
        (:`Is Not Valid`
          (message `/Game/Cards/BI_CardUser.CancelCardBeingUsed` _returnvalue_owneractor))))))

(event `self.MontageNotify`
  (params (NotifyIndex :type Integer))
  (bind _returnvalue (`self.GetOwningActorFromActorInfo`))
  (`self.RegenMana`)
  (bind _particleref (`self.SpawnParticleEffectsOnActor` (`self.GetOwningActorFromActorInfo`) "/Game/VFX/InfinityBladeEffects/Effects/FX_Cines/Ausar/P_Ausar_Resurrection.P_Ausar_Resurrection"))
  (set `self.Particle Ref` _particleref)
  (if (== (mod (`.ReturnValue` (`AbilitySystemBlueprintLibrary.GetFloatAttributeFromAbilitySystemComponent` (`self.GetAbilitySystemComponentFromActorInfo`) (struct :`AttributeName` "Health" :`Attribute` "/Script/CardGame.GAAttributeSet:Health" :`AttributeOwner` "/Script/CoreUObject.Class'\"/Script/CardGame.GAAttributeSet\"'"))) (`self.SecondMultiple`)) 0.0)
    (`|AddComponentByClass` _returnvalue "/Game/Components/BC_ApplyGEOverTime.BC_ApplyGEOverTime_C" (`self.AdditionalManaGained`) 3.0 0.2 "/Game/GAS/Effects/GE_RegenerateMana.GE_RegenerateMana_C" _returnvalue (struct :`TagName` "Mana.GainMana"))))

(event `self.MontageFinished`
  (bind _particle_ref (`self.Particle Ref`))
  (`AbilityTask_WaitDelay.WaitDelay` 2.0
    (:`OnFinish`
      (`/Engine/EditorBlueprintResources/StandardMacros.IsValid` _particle_ref
        (:`Is Valid`
          (`ActorComponent.K2_DestroyComponent` _particle_ref))
        (:`Is Not Valid`
          _))
      (`self.FinishAbility`))))