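; Gameplay ability for the Adrenaline Rush card, which restores mana and draws cards.
; It reads both amounts from the card's first ability entry, then plays a montage and waits for its notify.
; On the notify it grants and activates the regen-mana and draw-card abilities once each, passing the amounts as ability Level.
; It finishes after a short delay.
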(event `self.InitialiseCardStats`
  (bind (_gameplayability _description _amounts) (break `/Game/Cards/S_GA_Details` (`|GetArrayItem` (`.Abilities_64_195985E04BEB039D5D89D0BF920AEA2F` (break `/Game/Cards/S_CardInfo` (`self.CardInfo`))))))
  (set `self.TotalManaGained` (`|GetArrayItem` _amounts))
  (set `self.NumCardsToDraw` (`KismetMathLibrary.FTrunc` (`|GetArrayItem` _amounts 1))))

(event `self.K2_ActivateAbility`
  (`parent.K2_ActivateAbility`)
  (`self.PlayMontageAndWaitForNotify` "NewEnumerator11"))

(event `self.MontageNotify`
  (params (NotifyIndex :type Integer))
  (bind _returnvalue (`self.GetAbilitySystemComponentFromActorInfo`))
  (`AbilitySystemComponent.K2_GiveAbilityAndActivateOnce` _returnvalue "/Game/GAS/Abilities/RegenManaGA/GA_RegenManaGA.GA_RegenManaGA_C" (`KismetMathLibrary.FTrunc` (`self.TotalManaGained`)) -1)
  (`AbilitySystemComponent.K2_GiveAbilityAndActivateOnce` _returnvalue "/Game/GAS/Abilities/DrawCards/GA_DrawCardsGA.GA_DrawCardsGA_C" (`self.NumCardsToDraw`) -1)
  (`KismetSystemLibrary.Delay` 2.0)
  (`self.FinishAbility`))