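; GA_HealingTouch is a card-driven gameplay ability that heals its owner, reading both heal amounts from the card's info.
; On the montage notify it spawns a heal aura, spends card mana and applies the main amount through a gameplay effect.
; If the attribute ratio (presumably health to max) is below half, an added component also applies bonus healing over time.
; After the montage and a short delay, it removes the aura and finishes.
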(event `self.InitialiseCardStats`
  (bind (_cardinfo_name _cardinfo_image _cardinfo_description _cardinfo_backgroundcolour _cardinfo_abilities) (break `/Game/Cards/S_CardInfo` (`self.CardInfo`)))
  (bind (_gameplayability _description _amounts) (break `/Game/Cards/S_GA_Details` (`|GetArrayItem` _cardinfo_abilities)))
  (set `self.TotalAmountGained` (`|GetArrayItem` _amounts))
  (set `self.Additional Healing` (`|GetArrayItem` _amounts 1)))

(event `self.K2_ActivateAbility`
  (`parent.K2_ActivateAbility`)
  (`self.PlayMontageAndWaitForNotify` "NewEnumerator2"))

(event `self.MontageNotify`
  (params (NotifyIndex :type Integer))
  (bind _returnvalue (`self.GetOwningActorFromActorInfo`))
  (bind _returnvalue_2 (`self.GetAbilitySystemComponentFromActorInfo`))
  (bind _particleref (`self.SpawnParticleEffectsOnActor` (`self.GetOwningActorFromActorInfo`) "/Game/VFX/FXVarietyPack/Particles/P_ky_healAura.P_ky_healAura"))
  (set `self.Particle Ref` _particleref)
  (`self.UseCardMana`)
  (if (< (/ (`.ReturnValue` (`AbilitySystemBlueprintLibrary.GetFloatAttributeFromAbilitySystemComponent` _returnvalue_2 (struct :`AttributeName` "Health" :`Attribute` "/Script/CardGame.GAAttributeSet:Health" :`AttributeOwner` "/Script/CoreUObject.Class'\"/Script/CardGame.GAAttributeSet\"'"))) (`.ReturnValue` (`AbilitySystemBlueprintLibrary.GetFloatAttributeFromAbilitySystemComponent` _returnvalue_2 (struct :`AttributeName` "MaxHealth" :`Attribute` "/Script/CardGame.GAAttributeSet:MaxHealth" :`AttributeOwner` "/Script/CoreUObject.Class'\"/Script/CardGame.GAAttributeSet\"'")))) 0.5)
    (`|AddComponentByClass` _returnvalue "/Game/Components/BC_ApplyGEOverTime.BC_ApplyGEOverTime_C" (`self.Additional Healing`) 3.5 0.25 "/Game/GAS/Effects/GE_ChangeHealthBy.GE_ChangeHealthBy_C" _returnvalue (struct :`TagName` "Attribute.ChangeAmount")))
  (`self.ChangeAttributeOnActorByAmount` (`self.Gameplay Effect Class`) (`self.TotalAmountGained`) (`self.GetOwningActorFromActorInfo`)))

(event `self.MontageFinished`
  (bind _particle_ref (`self.Particle Ref`))
  (`AbilityTask_WaitDelay.WaitDelay` 2.0
    (:`OnFinish`
      (`/Engine/EditorBlueprintResources/StandardMacros.IsValid` _particle_ref
        (:`Is Valid`
          (`ActorComponent.K2_DestroyComponent` _particle_ref))
        (:`Is Not Valid`
          _))
      (`self.FinishAbility`))))