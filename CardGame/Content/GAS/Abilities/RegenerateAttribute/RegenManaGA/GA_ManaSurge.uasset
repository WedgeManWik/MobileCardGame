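; GA_ManaSurge is a card-based gameplay ability that grants mana to its owner, with a bonus when current mana is low.
; Base gain, mana threshold and bonus come from card data for the ability's level and upgrade state.
; On the montage notify, it applies a gameplay effect, adding the bonus below the threshold, and plays revive-style particles and sounds.
; After the montage and a short delay, it removes the particles and finishes.
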(event `self.InitialiseCardStats`
  (bind (_gameplayability _description _normalamounts _upgradedamounts _downgradedamounts) (break `/Game/Cards/S_GA_Details` (`|GetArrayItem` (`.Abilities_78_195985E04BEB039D5D89D0BF920AEA2F` (break `/Game/Cards/S_CardInfo` (`self.CardInfo`))) (`self.GetAbilityLevel`))))
  (bind _returnvalue (select `/Game/Cards/E_CardUpgradedState` (`self.Upgrade State`) :`NewEnumerator0` _normalamounts :`NewEnumerator1` _upgradedamounts :`NewEnumerator2` _downgradedamounts))
  (bind _output_amount (break `/Game/Cards/S_AmountType` (`|GetArrayItem` _returnvalue)))
  (bind _output_amount_2 (break `/Game/Cards/S_AmountType` (`|GetArrayItem` _returnvalue 1)))
  (bind _output_amount_3 (break `/Game/Cards/S_AmountType` (`|GetArrayItem` _returnvalue 2)))
  (set `self.TotalAmountGained` _output_amount)
  (set `self.MaxManaForBoost` (`KismetMathLibrary.FTrunc` _output_amount_2))
  (set `self.AdditionalManaGained` _output_amount_3))

(event `self.K2_ActivateAbility`
  (`self.InitialiseAbility`)
  (`self.PlayMontageAndWaitForNotify` "NewEnumerator2")
  (`GameplayStatics.PlaySound2D` "/Game/Audio/AbilitySFX/Bundle1/AMP_Buff_04.AMP_Buff_04" 1.0 1.0 0.0 null null))

(event `self.MontageNotify`
  (params (NotifyIndex :type Integer))
  (bind _returnvalue (`self.GetOwningActorFromActorInfo`))
  (bind _totalamountgained (`self.TotalAmountGained`))
  (`self.ChangeAttributeOnActorByAmount` (`self.Gameplay Effect Class`) (select `bool` (< (`KismetMathLibrary.FTrunc` (`.ReturnValue` (`AbilitySystemBlueprintLibrary.GetFloatAttributeFromAbilitySystemComponent` (`self.GetAbilitySystemComponentFromActorInfo`) (struct :`AttributeName` "Mana" :`Attribute` "/Script/CardGame.GAAttributeSet:Mana" :`AttributeOwner` "/Script/CoreUObject.Class'\"/Script/CardGame.GAAttributeSet\"'")))) (`self.MaxManaForBoost`)) :`false` _totalamountgained :`true` (+ _totalamountgained (`self.AdditionalManaGained`)) :!type "Float (single-precision)") _returnvalue)
  (bind _particleref (`self.SpawnParticleEffectsOnActor` _returnvalue "/Game/VFX/InfinityBladeEffects/Effects/FX_Cines/Ausar/P_Ausar_Resurrection.P_Ausar_Resurrection" false true))
  (set `self.Particle Ref` _particleref)
  (`GameplayStatics.PlaySound2D` "/Game/Audio/AbilitySFX/Magic_Attacks/Magic_Attacks/Arcane/Impact/Shine_Impact2.Shine_Impact2" 1.0 1.0 0.0 null null)
  (`GameplayStatics.PlaySound2D` "/Game/Audio/AbilitySFX/RW/703715__strangehorizon__magic_divine_revive.703715__strangehorizon__magic_divine_revive" 1.0 1.0 0.0 null null))

(event `self.MontageFinished`
  (params (`Finish Notify Index` :type Integer))
  (bind _particle_ref (`self.Particle Ref`))
  (`AbilityTask_WaitDelay.WaitDelay` 2.0
    (:`OnFinish`
      (`/Engine/EditorBlueprintResources/StandardMacros.IsValid` _particle_ref
        (:`Is Valid`
          (`ActorComponent.K2_DestroyComponent` _particle_ref))
        (:`Is Not Valid`
          _))
      (`self.FinishAbility`))))