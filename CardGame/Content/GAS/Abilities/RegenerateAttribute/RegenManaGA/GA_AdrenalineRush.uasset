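; GA_AdrenalineRush is a card gameplay ability that pairs a parent attribute gain, apparently mana regeneration, with card draw.
; Gain and draw amounts come from the card's ability data for the current level and upgrade state.
; Activation plays a montage, whose notify runs the parent activation and grants a one-shot GA_DrawCardsGA, passing the draw count as ability level.
; It finishes after a short delay.
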(event `self.InitialiseCardStats`
  (bind (_gameplayability _description _normalamounts _upgradedamounts _downgradedamounts) (break `/Game/Cards/S_GA_Details` (`|GetArrayItem` (`.Abilities_78_195985E04BEB039D5D89D0BF920AEA2F` (break `/Game/Cards/S_CardInfo` (`self.CardInfo`))) (`self.GetAbilityLevel`))))
  (bind _returnvalue (select `/Game/Cards/E_CardUpgradedState` (`self.Upgrade State`) :`NewEnumerator0` _normalamounts :`NewEnumerator1` _upgradedamounts :`NewEnumerator2` _downgradedamounts))
  (bind _output_amount (break `/Game/Cards/S_AmountType` (`|GetArrayItem` _returnvalue)))
  (bind _output_amount_2 (break `/Game/Cards/S_AmountType` (`|GetArrayItem` _returnvalue 1)))
  (set `self.TotalAmountGained` _output_amount)
  (set `self.NumCardsToDraw` (`KismetMathLibrary.FTrunc` _output_amount_2)))

(event `self.K2_ActivateAbility`
  (`self.PlayMontageAndWaitForNotify` "NewEnumerator11"))

(event `self.MontageNotify`
  (params (NotifyIndex :type Integer))
  (`parent.K2_ActivateAbility`)
  (`AbilitySystemComponent.K2_GiveAbilityAndActivateOnce` (`self.GetAbilitySystemComponentFromActorInfo`) "/Game/GAS/Abilities/DrawCards/GA_DrawCardsGA.GA_DrawCardsGA_C" (`self.NumCardsToDraw`) -1)
  (`KismetSystemLibrary.Delay` 2.0)
  (`self.FinishAbility`))