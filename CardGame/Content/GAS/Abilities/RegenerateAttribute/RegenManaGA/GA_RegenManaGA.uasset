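; Gameplay ability for cards that restores mana to its owner through the GE_RegenerateMana effect.
; InitialiseCardStats reads the gain amount from the card info when this is the card's only ability.
; On activation, a non-zero ability level overwrites that amount and triggers RegenMana; level zero applies nothing.
; RegenMana passes the amount as a Mana.GainMana SetByCaller magnitude on the effect spec it applies.
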(event `self.InitialiseCardStats`
  (bind (_cardinfo_name _cardinfo_image _cardinfo_description _cardinfo_backgroundcolour _cardinfo_abilities) (break `/Game/Cards/S_CardInfo` (`self.CardInfo`)))
  (bind (_gameplayability _description _amounts) (break `/Game/Cards/S_GA_Details` (`|GetArrayItem` _cardinfo_abilities)))
  (if (== (`KismetArrayLibrary.Array_Length` _cardinfo_abilities) 1)
    (if (== _gameplayability (`GameplayStatics.GetObjectClass` self))
      (set `self.TotalManaGained` (`|GetArrayItem` _amounts)))))

(event `self.K2_ActivateAbility`
  (bind _returnvalue (`self.GetAbilityLevel`))
  (`parent.K2_ActivateAbility`)
  (if (!= _returnvalue 0)
    (set `self.TotalManaGained` (`KismetMathLibrary.Conv_IntToDouble` _returnvalue))
    (`self.RegenMana`)))

(fn `RegenMana`
  (bind _returnvalue (`AbilitySystemBlueprintLibrary.AssignTagSetByCallerMagnitude` (`AbilitySystemComponent.MakeOutgoingSpec` :`self` (`self.GetAbilitySystemComponentFromActorInfo`) :`GameplayEffectClass` "/Game/GAS/Effects/GE_RegenerateMana.GE_RegenerateMana_C") (struct :`TagName` "Mana.GainMana") (`self.TotalManaGained`)))
  (`self.K2_ApplyGameplayEffectSpecToOwner` _returnvalue))