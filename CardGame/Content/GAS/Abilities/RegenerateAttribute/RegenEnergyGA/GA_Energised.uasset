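; GA_Energised is a card gameplay ability that restores energy to its owner, with a boost when energy is low.
; Amounts and threshold come from CardInfo by ability level and upgrade state.
; On montage notify it applies the gain, particles and sound, then repeats the same gain if the attribute remains below the threshold; AdditionalEnergyGained is never used.
; After the montage and a short delay, it removes the particles and finishes.
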(event `self.InitialiseCardStats`
  (bind (_gameplayability _description _normalamounts _upgradedamounts _downgradedamounts) (break `/Game/Cards/S_GA_Details` (`|GetArrayItem` (`.Abilities_78_195985E04BEB039D5D89D0BF920AEA2F` (break `/Game/Cards/S_CardInfo` (`self.CardInfo`))) (`self.GetAbilityLevel`))))
  (bind _returnvalue (select `/Game/Cards/E_CardUpgradedState` (`self.Upgrade State`) :`NewEnumerator0` _normalamounts :`NewEnumerator1` _upgradedamounts :`NewEnumerator2` _downgradedamounts))
  (bind _output_amount (break `/Game/Cards/S_AmountType` (`|GetArrayItem` _returnvalue)))
  (bind _output_amount_2 (break `/Game/Cards/S_AmountType` (`|GetArrayItem` _returnvalue 1)))
  (bind _output_amount_3 (break `/Game/Cards/S_AmountType` (`|GetArrayItem` _returnvalue 2)))
  (set `self.TotalAmountGained` _output_amount)
  (set `self.MaxEnergyForBoost` (`KismetMathLibrary.FTrunc` _output_amount_2))
  (set `self.AdditionalEnergyGained` _output_amount_3))

(event `self.K2_ActivateAbility`
  (`self.InitialiseAbility`)
  (`self.PlayMontageAndWaitForNotify` "NewEnumerator3"))

(event `self.MontageNotify`
  (params (NotifyIndex :type Integer))
  (bind _returnvalue (`self.GetOwningActorFromActorInfo`))
  (`self.ChangeAttributeOnActorByAmount` (`self.Gameplay Effect Class`) (`self.TotalAmountGained`) _returnvalue)
  (bind _particleref (`self.SpawnParticleEffectsOnActor` _returnvalue "/Game/VFX/InfinityBladeEffects/Effects/FX_Monsters/FX_Monster_Ausar/P_AU_ShieldSlam_AOE.P_AU_ShieldSlam_AOE" false true))
  (set `self.Particle Ref` _particleref)
  (`GameplayStatics.PlaySound2D` "/Game/Audio/AbilitySFX/RW/442872__qubodup__fire-magic.442872__qubodup__fire-magic" 1.0 1.0 0.0 null null)
  (if (< (`KismetMathLibrary.FTrunc` (`.ReturnValue` (`AbilitySystemBlueprintLibrary.GetFloatAttributeFromAbilitySystemComponent` (`self.GetAbilitySystemComponentFromActorInfo`) (struct :`AttributeName` "Energy" :`Attribute` "/Script/CardGame.GAAttributeSet:Energy" :`AttributeOwner` "/Script/CoreUObject.Class'\"/Script/CardGame.GAAttributeSet\"'")))) (`self.MaxEnergyForBoost`))
    (`self.ChangeAttributeOnActorByAmount` (`self.Gameplay Effect Class`) (`self.TotalAmountGained`) (`self.GetOwningActorFromActorInfo`))))

(event `self.MontageFinished`
  (params (`Finish Notify Index` :type Integer))
  (bind _particle_ref (`self.Particle Ref`))
  (`AbilityTask_WaitDelay.WaitDelay` 2.0
    (:`OnFinish`
      (`/Engine/EditorBlueprintResources/StandardMacros.IsValid` _particle_ref
        (:`Is Valid`
          (`ActorComponent.K2_DestroyComponent` _particle_ref))
        (:`Is Not Valid`
          _))
      (`self.FinishAbility`))))