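; Gameplay ability that regenerates an attribute by applying a gameplay effect to its owning actor.
; InitialiseCardStats sets TotalAmountGained from the card's first amount when this class is the card's only ability.
; On activation it runs the parent logic, then, if the ability level is nonzero, overwrites that amount with the level and passes it to ChangeAttributeOnActorByAmount.
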(event `self.InitialiseCardStats`
  (bind (_cardinfo_name _cardinfo_image _cardinfo_description _cardinfo_backgroundcolour _cardinfo_abilities) (break `/Game/Cards/S_CardInfo` (`self.CardInfo`)))
  (bind (_gameplayability _description _amounts) (break `/Game/Cards/S_GA_Details` (`|GetArrayItem` _cardinfo_abilities)))
  (if (== (`KismetArrayLibrary.Array_Length` _cardinfo_abilities) 1)
    (if (== _gameplayability (`GameplayStatics.GetObjectClass` self))
      (set `self.TotalAmountGained` (`|GetArrayItem` _amounts)))))

(event `self.K2_ActivateAbility`
  (bind _returnvalue (`self.GetAbilityLevel`))
  (`parent.K2_ActivateAbility`)
  (if (!= _returnvalue 0)
    (bind _output_get (set `self.TotalAmountGained` (`KismetMathLibrary.Conv_IntToDouble` _returnvalue)))
    (`self.ChangeAttributeOnActorByAmount` (`self.Gameplay Effect Class`) _output_get (`self.GetOwningActorFromActorInfo`))))