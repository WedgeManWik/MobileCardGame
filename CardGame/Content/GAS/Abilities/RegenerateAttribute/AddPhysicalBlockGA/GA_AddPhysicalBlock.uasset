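; Gameplay Ability for a card that grants Physical Block to its owner.
; On activation it reads the gained amount from the card's ability data, selected by level and Normal, Upgraded or Downgraded state.
; It then calls Regenerate, pays the card cost, spawns floaty text with the amount, plays an armor-up sound and finishes after a brief delay.
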(event `self.K2_ActivateAbility`
  (bind (_cardinfo_name _cardinfo_image _cardinfo_description _cardinfo_backgroundcolour _cardinfo_abilities) (break `/Game/Cards/S_CardInfo` (`self.CardInfo`)))
  (bind (_output_gameplayability _output_description _output_normalamounts _output_upgradedamounts _output_downgradedamounts) (break `/Game/Cards/S_GA_Details` (`|GetArrayItem` _cardinfo_abilities (`self.GetAbilityLevel`))))
  (`self.InitialiseAbility`)
  (for _array_element (select `/Game/Cards/E_CardUpgradedState` (`self.Upgrade State`) :`NewEnumerator0` _output_normalamounts :`NewEnumerator1` _output_upgradedamounts :`NewEnumerator2` _output_downgradedamounts)
    (bind (_amount _type) (break `/Game/Cards/S_AmountType` _array_element))
    (if (`|EnumEquality` _type "NewEnumerator8")
      (set `self.TotalAmountGained` _amount)))
  (`self.Regenerate`)
  (`self.UseCardCost`)
  (`|SpawnActorFromClass` "/Game/UI/FloatyText/BP_FloatyText.BP_FloatyText_C" (`KismetMathLibrary.Conv_VectorToTransform` (`Actor.K2_GetActorLocation` (`self.GetOwningActorFromActorInfo`))) "Undefined" "MultiplyWithRoot" null (`KismetStringLibrary.Concat_StrStr` "+ " (`KismetStringLibrary.Conv_DoubleToString` (`self.TotalAmountGained`)) "Physical Block") null)
  (`GameplayStatics.PlaySound2D` "/Game/Audio/CardsSFX/Buff/GP_Armor_Up_1.GP_Armor_Up_1" 1.0 1.0 0.0 null null)
  (`KismetSystemLibrary.Delay` 0.2)
  (`self.FinishAbility`))

(event `self.K2_OnEndAbility`
  (params (bWasCancelled :type Boolean))
  (`parent.K2_OnEndAbility` bWasCancelled))