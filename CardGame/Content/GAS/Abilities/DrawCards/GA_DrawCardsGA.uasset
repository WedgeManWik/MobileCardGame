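; Gameplay ability that makes its owner draw cards, using the ability level as the number of cards.
; On activation it sends DrawCardsMessage with that count to the PlayerController from the actor info, or to the owner actor when no valid controller exists.
; The ability finishes immediately after sending the message.
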(event `self.K2_ActivateAbility`
  (`parent.K2_ActivateAbility`)
  (`self.Draw` (`self.GetAbilityLevel`)))

(event `Draw`
  (params (`Card Amount` :type Integer))
  (bind (_returnvalue_owneractor _returnvalue_avataractor _returnvalue_playercontroller) (break `GameplayAbilityActorInfo` (`self.GetActorInfo`)))
  (message `/Game/Cards/BI_CardUser.DrawCards` (`KismetMathLibrary.SelectObject` _returnvalue_playercontroller _returnvalue_owneractor (`KismetSystemLibrary.IsValid` _returnvalue_playercontroller)) `Card Amount`)
  (`self.FinishAbility`))