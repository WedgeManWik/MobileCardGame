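; Gameplay ability for the Battle Tactics card, which draws cards and draws extra when the hand count is exactly one.
; Base and bonus draw amounts come from the card's ability data for the current level.
; Activation pays the card cost, waits briefly, then queries hand size through a message to the PlayerController, falling back to the owner actor when no controller is valid.
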(event `self.InitialiseCardStats`
  (bind (_cardinfo_name _cardinfo_image _cardinfo_description _cardinfo_backgroundcolour _cardinfo_abilities) (break `/Game/Cards/S_CardInfo` (`self.CardInfo`)))
  (bind (_gameplayability _description _amounts) (break `/Game/Cards/S_GA_Details` (`|GetArrayItem` _cardinfo_abilities (`self.GetAbilityLevel`))))
  (set `self.Amount Cards Gained` (`KismetMathLibrary.FTrunc` (`|GetArrayItem` _amounts)))
  (set `self.Extra Cards Gained` (`KismetMathLibrary.FTrunc` (`|GetArrayItem` _amounts 1))))

(event `self.K2_ActivateAbility`
  (bind (_returnvalue_owneractor _returnvalue_avataractor _returnvalue_playercontroller) (break `GameplayAbilityActorInfo` (`self.GetActorInfo`)))
  (bind _amount_cards_gained (`self.Amount Cards Gained`))
  (`self.InitialiseAbility`)
  (`self.UseCardCost`)
  (`KismetSystemLibrary.Delay` 0.2)
  (bind _num_cards_in_hand (message `/Game/Cards/BI_CardUser.GetNumCardsInHand` (`KismetMathLibrary.SelectObject` _returnvalue_playercontroller _returnvalue_owneractor (`KismetSystemLibrary.IsValid` _returnvalue_playercontroller))))
  (`self.Draw` (`KismetMathLibrary.SelectInt` (+ (`self.Extra Cards Gained`) _amount_cards_gained) _amount_cards_gained (== _num_cards_in_hand 1))))