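; GA_HealGA is a Gameplay Ability that heals its owner by an amount equal to the ability level.
; On activation with a non-zero level, it stores the level as TotalHealAmount and calls Heal.
; Heal builds a GE_Heal spec, sets the amount as a SetByCaller magnitude under Event.Heal and applies it to the owner.
; The graph never calls EndAbility.
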(event `self.K2_ActivateAbility`
  (bind _returnvalue (`self.GetAbilityLevel`))
  (`parent.K2_ActivateAbility`)
  (if (!= _returnvalue 0)
    (set `self.TotalHealAmount` (`KismetMathLibrary.Conv_IntToDouble` _returnvalue))
    (`self.Heal`)))

(fn `Heal`
  (bind _returnvalue (`AbilitySystemBlueprintLibrary.AssignTagSetByCallerMagnitude` (`AbilitySystemComponent.MakeOutgoingSpec` :`self` (`self.GetAbilitySystemComponentFromActorInfo`) :`GameplayEffectClass` "/Game/GAS/Effects/GE_Heal.GE_Heal_C") (struct :`TagName` "Event.Heal") (`self.TotalHealAmount`)))
  (`self.K2_ApplyGameplayEffectSpecToOwner` _returnvalue))