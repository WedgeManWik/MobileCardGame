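; Player character for turn-based, card-driven combat, built on a parent character class with the Gameplay Ability System.
; Adds a health bar and, when attack or defence attributes change, updates the combat stats widget and refreshes every player card's ability description.
; Relays turn and target-selection calls to the controller and gets enemies from the game mode through messages.
; An unconnected chain for stat-based health change and mana/energy regen never runs.
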(event `self.OnMagicAttackChanged`
  (params (OldValue :type "Float (single-precision)") (NewValue :type "Float (single-precision)"))
  (`/Game/UI/StatusBars/WB_CharacterCombatStats.SetAttribute` (`/Game/UI/StatusBars/WB_CharacterStatBar.WB_CharacterCombatStats` (`self.StatBars`)) (struct :`AttributeName` "MagicAttack" :`Attribute` "/Script/CardGame.GAAttributeSet:MagicAttack" :`AttributeOwner` "/Script/CoreUObject.Class'\"/Script/CardGame.GAAttributeSet\"'") OldValue NewValue 0.0)
  (bind _cards (message `/Game/GameModes/BI_GameInstance.GetPlayerCards` (`GameplayStatics.GetGameInstance`) :!label _label))
  (for _array_element _cards
    (`/Game/Cards/WB_Card.SetAbilityDescriptionText` _array_element)))

(event `self.InitialiseHealthBars`
  (bind _abilitysystemcomponent (`self.AbilitySystemComponent`))
  (`KismetSystemLibrary.DelayUntilNextTick`)
  (`/Game/UI/StatusBars/WB_CharacterStatBar.AddBar` (`self.StatBars`) "Health" (struct :`G` 1.0 :`A` 1.0) (`.ReturnValue` (`AbilitySystemBlueprintLibrary.GetFloatAttributeFromAbilitySystemComponent` _abilitysystemcomponent (struct :`AttributeName` "Health" :`Attribute` "/Script/CardGame.GAAttributeSet:Health" :`AttributeOwner` "/Script/CoreUObject.Class'\"/Script/CardGame.GAAttributeSet\"'"))) (`.ReturnValue` (`AbilitySystemBlueprintLibrary.GetFloatAttributeFromAbilitySystemComponent` _abilitysystemcomponent (struct :`AttributeName` "MaxHealth" :`Attribute` "/Script/CardGame.GAAttributeSet:MaxHealth" :`AttributeOwner` "/Script/CoreUObject.Class'\"/Script/CardGame.GAAttributeSet\"'"))) false)
  (`parent.InitialiseHealthBars`))

(event `self.OnMagicDefenceChanged`
  (params (OldValue :type "Float (single-precision)") (NewValue :type "Float (single-precision)"))
  (`/Game/UI/StatusBars/WB_CharacterCombatStats.SetAttribute` (`/Game/UI/StatusBars/WB_CharacterStatBar.WB_CharacterCombatStats` (`self.StatBars`)) (struct :`AttributeName` "MagicDefence" :`Attribute` "/Script/CardGame.GAAttributeSet:MagicDefence" :`AttributeOwner` "/Script/CoreUObject.Class'\"/Script/CardGame.GAAttributeSet\"'") OldValue NewValue 0.0)
  (goto _label))

(event `self.OnPhysicalAttackChanged`
  (params (OldValue :type "Float (single-precision)") (NewValue :type "Float (single-precision)"))
  (`/Game/UI/StatusBars/WB_CharacterCombatStats.SetAttribute` (`/Game/UI/StatusBars/WB_CharacterStatBar.WB_CharacterCombatStats` (`self.StatBars`)) (struct :`AttributeName` "PhysicalAttack" :`Attribute` "/Script/CardGame.GAAttributeSet:PhysicalAttack" :`AttributeOwner` "/Script/CoreUObject.Class'\"/Script/CardGame.GAAttributeSet\"'") OldValue NewValue 0.0)
  (goto _label))

(event `self.ReceiveBeginPlay`
  (`parent.ReceiveBeginPlay`))

(event `self.OnPhysicalDefenceChanged`
  (params (OldValue :type "Float (single-precision)") (NewValue :type "Float (single-precision)"))
  (`/Game/UI/StatusBars/WB_CharacterCombatStats.SetAttribute` (`/Game/UI/StatusBars/WB_CharacterStatBar.WB_CharacterCombatStats` (`self.StatBars`)) (struct :`AttributeName` "PhysicalDefence" :`Attribute` "/Script/CardGame.GAAttributeSet:PhysicalDefence" :`AttributeOwner` "/Script/CoreUObject.Class'\"/Script/CardGame.GAAttributeSet\"'") OldValue NewValue 0.0)
  (goto _label))

(event `/Game/Cards/BI_CardUser.StartTurn`
  (`parent.StartTurn`))

(event `self.FinishedDeathAnimation`)

(event `/Game/Cards/BI_CardUser.EndTurn`
  (message `/Game/Cards/BI_CardUser.EndTurn` (`self.GetController`)))

(event `self.TurnStart`
  (message `/Game/Cards/BI_CardUser.StartTurn` (`self.GetController`)))

(event `/Game/Cards/BI_CardUser.SetSelectedTargets`
  (params (SelectedTargets :type "Array of Actor Object Reference (by ref)"))
  (message `/Game/Cards/BI_CardUser.SetSelectedTargets` (`self.GetController`) SelectedTargets))

(fn `GetAllEnemies`
  (returns (Enemies :type "Array of Actor Object Reference"))
  (bind _enemies (message `/Game/GameModes/BI_CardGameMode.GetAllEnemies` (`GameplayStatics.GetGameMode`)))
  (return _enemies))

(fn `GetSelectedTargets`
  (returns (Targets :type "Array of Actor Object Reference"))
  (bind _targets (message `/Game/Cards/BI_CardUser.GetSelectedTargets` (`self.GetController`)))
  (return _targets))

(fn `UserConstructionScript`
  (`parent.UserConstructionScript`))