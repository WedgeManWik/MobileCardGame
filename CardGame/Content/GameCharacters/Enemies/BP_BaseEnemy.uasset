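; Base enemy for a turn-based card game, which plays a random card on its turn through the Gameplay Ability System.
; StartTurn waits briefly, picks a random DT_Cards row, sets the card in use and gives and activates its first ability once.
; Target selection immediately sends itself a TargetsSet gameplay event, with the player stored as its target at BeginPlay.
; When the card has been used, it notifies the game mode that its turn is finished.
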(event `self.ReceiveBeginPlay`
  (`KismetArrayLibrary.Array_Add` (`self.Targets`) (`GameplayStatics.GetPlayerCharacter` 0)))

(event `/Game/Cards/BI_CardUser.StartTurn`
  (`KismetSystemLibrary.Delay` 1.0)
  (bind _outrownames (`DataTableFunctionLibrary.GetDataTableRowNames` "/Game/Cards/DT_Cards.DT_Cards"))
  (bind _returnvalue (`|GetDataTableRow` "/Game/Cards/DT_Cards.DT_Cards" (`KismetArrayLibrary.Array_Random` _outrownames))
    (:`then`
      (bind (_name _image _description _backgroundcolour _abilities _manacost _cardid) (break `/Game/Cards/S_CardInfo` _returnvalue))
      (message `/Game/Cards/BI_CardUser.SetCardBeingUsed` self _cardid null)
      (`AbilitySystemComponent.K2_GiveAbilityAndActivateOnce` (`self.AbilitySystemComponent`) (`|GetArrayItem` _abilities) 0 -1))))

(event `/Game/Cards/BI_CardUser.SelectTargetsToUseOnCard`
  (params (MaxNumTargets :type Integer))
  (`AbilitySystemBlueprintLibrary.SendGameplayEventToActor` self (struct :`TagName` "Action.TargetsSet") (make `GameplayEventData` (struct :`TagName` "Action.TargetsSet"))))

(event `/Game/Cards/BI_CardUser.CardHasBeenUsed`
  (message `/Game/TopDown/Blueprints/BI_CardGameMode.FinishedTurn` (`GameplayStatics.GetGameMode`)))

(fn `GetAllEnemies`
  (returns (Enemies :type "Array of Actor Object Reference"))
  (return (`self.Targets`)))

(fn `UserConstructionScript`)