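; PC_Win is the player controller for the win screen.
; On BeginPlay it waits a tick, switches the view to a CameraActor found in the level, adds the WB_WinScreen widget and plays music.
; It then messages the controlled pawn to hide its UI and, after a short delay, to play a montage.
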(event `self.ReceiveBeginPlay`
  (bind _returnvalue (`self.K2_GetPawn`))
  (`KismetSystemLibrary.DelayUntilNextTick`)
  (bind _returnvalue_2 (`GameplayStatics.GetActorOfClass` "/Script/Engine.CameraActor"))
  (`self.SetViewTargetWithBlend` self _returnvalue_2 0.0 "VTBlend_Linear" 0.0 false)
  (bind _returnvalue_3 (`|CreateWidget` "/Game/UI/Menus/WinScreen/WB_WinScreen.WB_WinScreen_C"))
  (`UserWidget.AddToViewport` _returnvalue_3 0)
  (`GameplayStatics.PlaySound2D` "/Game/Audio/Music/Pack2/Medieval_Vol__2_6.Medieval_Vol__2_6" 1.0 1.0 1.5 null null)
  (message `/Game/Cards/BI_CardUser.HideUI` _returnvalue)
  (`KismetSystemLibrary.Delay` 1.0)
  (message `/Game/Cards/BI_CardUser.PlayMontage` _returnvalue "NewEnumerator21" 1.0))

(fn `UserConstructionScript`)