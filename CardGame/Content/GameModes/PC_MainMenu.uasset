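; Player controller for the main menu that manages the main, character selection and deck-building screens and starts UI-only on the main menu.
; Each load function removes all menus, lazily creates and caches its widget, binds that widget's navigation events, then adds it to the player screen.
; PlayGame leaves the menus by opening the LevelSelection level.
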(event `self.ReceiveBeginPlay`
  (`self.LoadMainMenu`)
  (`WidgetBlueprintLibrary.SetInputMode_UIOnlyEx` self null))

(fn `LoadCharacterSelectionMenu`
  (`self.UnloadMenus`)
  (`/Engine/EditorBlueprintResources/StandardMacros.IsValid` (`self.CharacterSelectionMenu`)
    (:`Is Valid`
      _)
    (:`Is Not Valid`
      (bind _returnvalue (`|CreateWidget` "/Game/UI/Menus/WB_CharacterSelection.WB_CharacterSelection_C" self))
      (bind _output_get (set `self.CharacterSelectionMenu` _returnvalue))
      (add `/Game/UI/Menus/WB_CharacterSelection.OnBackToMainMenu` _output_get (`|CreateDelegate` :!event `LoadMainMenu`))
      (add `/Game/UI/Menus/WB_CharacterSelection.OnConfirmedCharacter` _output_get (`|CreateDelegate` :!event `LoadDeckBuildingMenu`))))
  (`UserWidget.AddToPlayerScreen` (`self.CharacterSelectionMenu`) 0))

(fn `LoadDeckBuildingMenu`
  (`self.UnloadMenus`)
  (`/Engine/EditorBlueprintResources/StandardMacros.IsValid` (`self.DeckBuildMenu`)
    (:`Is Valid`
      _)
    (:`Is Not Valid`
      (bind _returnvalue (`|CreateWidget` "/Game/UI/Menus/WB_DeckBuild.WB_DeckBuild_C" self))
      (bind _output_get (set `self.DeckBuildMenu` _returnvalue))
      (add `/Game/UI/Menus/WB_DeckBuild.OnPlay` _output_get (`|CreateDelegate` :!event `PlayGame`))
      (add `/Game/UI/Menus/WB_DeckBuild.OnBackToCharacterSelection` _output_get (`|CreateDelegate` :!event `LoadCharacterSelectionMenu`))))
  (`UserWidget.AddToPlayerScreen` (`self.DeckBuildMenu`) 0))

(fn `LoadMainMenu`
  (`self.UnloadMenus`)
  (`/Engine/EditorBlueprintResources/StandardMacros.IsValid` (`self.MainMenu`)
    (:`Is Valid`
      _)
    (:`Is Not Valid`
      (bind _returnvalue (`|CreateWidget` "/Game/UI/Menus/WB_MainMenu.WB_MainMenu_C" self))
      (bind _output_get (set `self.MainMenu` _returnvalue))
      (add `/Game/UI/Menus/WB_MainMenu.OnPlay` _output_get (`|CreateDelegate` :!event `LoadCharacterSelectionMenu`))))
  (`UserWidget.AddToPlayerScreen` (`self.MainMenu`) 0))

(fn `PlayGame`
  (`GameplayStatics.OpenLevelBySoftObjectPtr` "/Game/TopDown/Maps/LevelSelection.LevelSelection"))

(fn `UnloadMenus`
  (bind _mainmenu (`self.MainMenu`))
  (bind _characterselectionmenu (`self.CharacterSelectionMenu`))
  (bind _deckbuildmenu (`self.DeckBuildMenu`))
  (`/Engine/EditorBlueprintResources/StandardMacros.IsValid` _mainmenu
    (:`Is Valid`
      (`Widget.RemoveFromParent` _mainmenu))
    (:`Is Not Valid`
      _))
  (`/Engine/EditorBlueprintResources/StandardMacros.IsValid` _characterselectionmenu
    (:`Is Valid`
      (`Widget.RemoveFromParent` _characterselectionmenu))
    (:`Is Not Valid`
      _))
  (`/Engine/EditorBlueprintResources/StandardMacros.IsValid` _deckbuildmenu
    (:`Is Valid`
      (`Widget.RemoveFromParent` _deckbuildmenu))))

(fn `UserConstructionScript`)