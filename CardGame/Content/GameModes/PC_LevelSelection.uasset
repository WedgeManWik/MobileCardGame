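; Player controller for the level-selection map, handling map navigation and what happens when the player enters a room.
; When the BP_MapPawn reports an entered room, it saves the room ID to the game instance, then loads the cave level for enemy encounters or shows the matching card swap, shop, camp or workshop widget.
; Enhanced Input touch and zoom actions message the pawn with swipe and pinch-distance deltas, with zoom using mouse position on Windows.
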(event `self.ReceiveBeginPlay`
  (`WidgetBlueprintLibrary.SetInputMode_GameAndUIEx` self null "DoNotLock" false)
  (`EnhancedInputSubsystemInterface.AddMappingContext` (subsystem `EnhancedInputLocalPlayerSubsystem`) "/Game/GameCharacters/Player/Input/IMC_Player.IMC_Player" 0 (struct))
  (bind _asbp_map_pawn (cast `/Game/GameModes/BP_MapPawn` (`self.K2_GetPawn`)))
  (add `/Game/GameModes/BP_MapPawn.OnEnteredRoom` _asbp_map_pawn (delegate `EnteredRoom`)))

(event `EnteredRoom`
  (params (RoomID :type Integer) (RoomType :type "/Game/UI/Menus/LevelSelection/E_RoomType Enum" :default "NewEnumerator0"))
  (message `/Game/GameModes/BI_Map.SetCurrentRoomID` (`GameplayStatics.GetGameInstance`) RoomID)
  (switch `/Game/UI/Menus/LevelSelection/E_RoomType` RoomType
    (:`NewEnumerator1`
      (`GameplayStatics.OpenLevelBySoftObjectPtr` "/Game/SoulCave/Maps/LV_Soul_Cave_Mobile.LV_Soul_Cave_Mobile"))
    (:`NewEnumerator2`
      (bind _returnvalue (`|CreateWidget` "/Game/UI/Menus/CardSwap/WB_CardSwap.WB_CardSwap_C" self))
      (`UserWidget.AddToViewport` _returnvalue 0))
    (:`NewEnumerator3`
      (bind _returnvalue_2 (`|CreateWidget` "/Game/UI/Menus/RewardScreen/ItemEquip/WB_EquipItem.WB_EquipItem_C"))
      (`UserWidget.AddToViewport` _returnvalue_2 0))
    (:`NewEnumerator4`
      (bind _returnvalue_3 (`|CreateWidget` "/Game/UI/Menus/Camp/WB_Camp.WB_Camp_C" self))
      (`UserWidget.AddToViewport` _returnvalue_3 0))
    (:`NewEnumerator5`
      (bind _returnvalue_4 (`|CreateWidget` "/Game/UI/Menus/Workshop/WB_Workshop.WB_Workshop_C" self))
      (`UserWidget.AddToViewport` _returnvalue_4 0))))

(event `EnhancedInput|/Game/GameCharacters/Player/Input/IA_Touch`
  (params (ActionValue :type Boolean) (ElapsedSeconds :type "Float (double-precision)") (TriggeredSeconds :type "Float (double-precision)") (InputAction :type "InputAction Object Reference" :default "/Game/GameCharacters/Player/Input/IA_Touch.IA_Touch"))
  (bind (_locationx _locationy) (`self.GetInputTouchState` "Touch1"))
  (bind (_locationx_2 _locationy_2) (`self.GetInputTouchState` "Touch1"))
  (bind _returnvalue (`KismetMathLibrary.MakeVector2D` _locationx _locationy))
  (:`Triggered`
    (message `/Game/GameModes/BI_Map.PanMap` (`self.K2_GetPawn`) (- _returnvalue (`self.StartSwipeLocation`)))
    (set `self.StartSwipeLocation` _returnvalue))
  (:`Started`
    (set `self.StartSwipeLocation` (`KismetMathLibrary.MakeVector2D` _locationx_2 _locationy_2))))

(event `EnhancedInput|/Game/GameCharacters/Player/Input/IA_Zoom`
  (params (ActionValue :type Boolean) (ElapsedSeconds :type "Float (double-precision)") (TriggeredSeconds :type "Float (double-precision)") (InputAction :type "InputAction Object Reference" :default "/Game/GameCharacters/Player/Input/IA_Zoom.IA_Zoom"))
  (:`Triggered`
    (message `/Game/GameModes/BI_Map.ZoomOnMap` (`self.K2_GetPawn`) (- (`self.StartZoomTouchDistance`) (`self.Get Touch Distance`))))
  (:`Started`
    (set `self.StartZoomTouchDistance` (`self.Get Touch Distance`))))

(fn `Get Touch Distance`
  (returns (Distance :type "Float (double-precision)"))
  (bind (_locationx _locationy) (`self.GetMousePosition`))
  (bind (_locationx_2 _locationy_2) (`self.GetInputTouchState` "Touch2"))
  (bind (_locationx_3 _locationy_3) (`self.GetInputTouchState` "Touch1"))
  (return (`KismetMathLibrary.VSize2D` (select `bool` (`KismetStringLibrary.EqualEqual_StrStr` (`GameplayStatics.GetPlatformName`) "Windows") :`false` (- (`KismetMathLibrary.MakeVector2D` _locationx_3 _locationy_3) (`KismetMathLibrary.MakeVector2D` _locationx_2 _locationy_2)) :`true` (`KismetMathLibrary.MakeVector2D` _locationx _locationy)))))

(fn `UserConstructionScript`)