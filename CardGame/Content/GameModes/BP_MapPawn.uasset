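; BP_MapPawn is the map screen pawn, holding a fixed set of child-actor room icons with spring-arm zoom and panning.
; BeginPlay gathers the rooms, binds their press events and restores the current room from the GameInstance.
; Clicks move only to connected rooms, or to a Start Point when none is current, then fire OnEnteredRoom.
; Connection IDs index the Rooms array to toggle which neighbors are enterable.
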(event `self.ReceiveBeginPlay`
  (for _array_element (`|MakeArray` (`self.Room_0`) (`self.Room_1`) (`self.Room_2`) (`self.Room_3`) (`self.Room_4`) (`self.Room_5`) (`self.Room_6`) (`self.Room_7`) (`self.Room_8`) (`self.Room_9`) (`self.Room_10`) (`self.Room_11`) (`self.Room_12`) (`self.Room_13`) (`self.Room_14`) (`self.Room_15`) (`self.Room_16`) (`self.Room_17`) (`self.Room_18`) (`self.Room_19`) (`self.Room_20`) (`self.Room_21`) (`self.Room_22`) (`self.Room_23`) (`self.Room_24`) (`self.Room_25`) (`self.Room_26`) (`self.Room_27`) (`self.Room_28`) (`self.Room_29`) (`self.Room_30`) (`self.Room_31`) (`self.Room_32`) (`self.Room_33`) (`self.Room_34`) (`self.Room_35`) (`self.Room_36`) (`self.Room_37`) (`self.Room_38`) (`self.Room_39`) (`self.Room_40`) (`self.Room_41`) (`self.Room_42`) (`self.Room_43`) (`self.Room_44`) (`self.Room_45`) (`self.Room_46`) (`self.Room_47`) (`self.Room_48`) (`self.Room_49`) (`self.Room_50`) (`self.Room_51`) (`self.Room_52`) (`self.Room_53`) (`self.Room_54`) (`self.Room_55`) (`self.Room_56`) (`self.Room_57`) (`self.Room_58`) (`self.Room_59`) (`self.Room_60`) (`self.Room_61`) (`self.Room_62`) (`self.Room_63`) (`self.Room_64`) (`self.Room_65`) (`self.Room_66`) (`self.Room_67`) (`self.Room_68`) (`self.Room_69`) (`self.Room_70`) (`self.Room_71`) (`self.Room_72`) (`self.Room_73`) (`self.Room_74`) (`self.Room_75`) (`self.Room_76`))
    (bind _childactor (`ChildActorComponent.ChildActor` _array_element))
    (`KismetArrayLibrary.Array_Add` (`self.Rooms`) _childactor)
    (bind _asbp_room_icon (cast `/Game/UI/Menus/LevelSelection/BP_RoomIcon` _childactor))
    (add `/Game/UI/Menus/LevelSelection/BP_RoomIcon.OnPressed` _asbp_room_icon (`|CreateDelegate` :!event `RoomClicked`)))
  (bind _roomid (message `/Game/GameModes/BI_Map.GetCurrentRoomID` (`GameplayStatics.GetGameInstance`)))
  (`self.SetCurrentRoomID` _roomid))

(event `RoomClicked`
  (params (RoomRef :type "/Game/UI/Menus/LevelSelection/BP_RoomIcon Object Reference"))
  (`/Engine/EditorBlueprintResources/StandardMacros.IsValid` (`self.CurrentRoom`)
    (:`Is Valid`
      (bind _roomconnections (message `/Game/UI/Menus/LevelSelection/BI_RoomIcon.GetConnections` (`self.CurrentRoom`)))
      (for _array_element _roomconnections
        (if (== _array_element (`/Game/UI/Menus/LevelSelection/BP_RoomIcon.ID` RoomRef))
          (`self.MoveToNextRoom` RoomRef))))
    (:`Is Not Valid`
      (switch `/Game/UI/Menus/LevelSelection/E_RoomType` (`/Game/UI/Menus/LevelSelection/BP_RoomIcon.RoomType` RoomRef)
        (:`NewEnumerator0`
          (`self.MoveToNextRoom` RoomRef))))))

(event `MoveToNextRoom`
  (params (NextRoom :type "/Game/UI/Menus/LevelSelection/BP_RoomIcon Object Reference"))
  (bind _currentroom (`self.CurrentRoom`))
  (`/Engine/EditorBlueprintResources/StandardMacros.IsValid` _currentroom
    (:`Is Valid`
      (`self.SetIsCurrentRoom` _currentroom))
    (:`Is Not Valid`
      _))
  (bind _output_get (set `self.CurrentRoom` NextRoom))
  (`self.SetIsCurrentRoom` _output_get true)
  (bind (_id _roomtype) (message `/Game/UI/Menus/LevelSelection/BI_RoomIcon.GetRoomInfo` (`self.CurrentRoom`)))
  (`self.OnEnteredRoom` _id _roomtype))

(event `self.ZoomOnMap`
  (params (ZoomAmount :type "Float (double-precision)"))
  (bind _springarm (`self.SpringArm`))
  (set `SpringArmComponent.TargetArmLength` (`KismetMathLibrary.FClamp` (+ (`SpringArmComponent.TargetArmLength` _springarm) (* ZoomAmount (`self.ZoomSensitivity`))) 500.0 2000.0) _springarm))

(event `SetIsCurrentRoom`
  (params (Room :type "Actor Object Reference") (IsCurrentRoom :type Boolean))
  (message `/Game/UI/Menus/LevelSelection/BI_RoomIcon.SetAsCurrentRoom` Room IsCurrentRoom)
  (bind _roomconnections (message `/Game/UI/Menus/LevelSelection/BI_RoomIcon.GetConnections` Room))
  (for _array_element _roomconnections
    (message `/Game/UI/Menus/LevelSelection/BI_RoomIcon.SetAsEnterable` (`|GetArrayItem` (`self.Rooms`) _array_element) IsCurrentRoom)))

(event `self.PanMap`
  (params (Translation :type "Vector2D Structure"))
  (bind _springarm (`self.SpringArm`))
  (`SceneComponent.K2_SetRelativeLocation` _springarm (- (`SceneComponent.RelativeLocation` _springarm) (* (`KismetMathLibrary.MakeVector` 0.0 Translation_X (* Translation_Y -1.0)) (`self.PanSensitivity`))) false true))

(event `self.SetCurrentRoomID`
  (params (ID :type Integer))
  (bind _output_get (set `self.CurrentRoom` (`|GetArrayItem` (`self.Rooms`) ID)))
  (`self.SetIsCurrentRoom` _output_get true))

(fn `GetCurrentRoomID`
  (returns (RoomID :type Integer))
  (return 0))

(fn `GetNumRoomsEntered`
  (returns (NumRoomsEntered :type Integer))
  (return 0))

(fn `UserConstructionScript`)