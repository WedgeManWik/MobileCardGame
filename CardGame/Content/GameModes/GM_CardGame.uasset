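; Game mode for a turn-based card game that runs the turn order between the player and enemies.
; After a short delay on BeginPlay, it builds a roster of the player followed by every BI_Enemy actor, then starts the first turn.
; FinishedTurn sends a gameplay event, advances the index and counts rounds on wrap; CharacterDied removes actors from the lists.
; The default pawn class comes from the GameInstance's selected character, falling back to the parent's.
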(event `self.ReceiveBeginPlay`
  (bind _characters (`self.Characters`))
  (`KismetSystemLibrary.Delay` 0.2)
  (bind _outactors (`GameplayStatics.GetAllActorsWithInterface` "/Game/GameCharacters/Enemies/BI_Enemy.BI_Enemy_C"))
  (bind _output_get (set `self.Enemies` _outactors))
  (`KismetArrayLibrary.Array_Add` _characters (`GameplayStatics.GetPlayerCharacter` 0))
  (for _array_element _output_get
    (`KismetArrayLibrary.Array_Add` _characters _array_element))
  (message `/Game/Cards/BI_CardUser.StartTurn` (`|GetArrayItem` (`self.Characters`))))

(event `/Game/GameModes/BI_CardGameMode.FinishedTurn`
  (params (Actor :type "Actor Object Reference"))
  (`AbilitySystemBlueprintLibrary.SendGameplayEventToActor` Actor (struct :`TagName` "Event.Turn.Finished") (make `GameplayEventData` (struct :`TagName` "Event.Turn.Finished")))
  (bind _result (`/Engine/EditorBlueprintResources/StandardMacros.IncrementInt` (`self.CharacterTurnIndex`))
    (:`  `
      (if (>= _result (`KismetArrayLibrary.Array_Length` (`self.Characters`)))
        (set `self.CharacterTurnIndex` 0)
        (bind _result_2 (`/Engine/EditorBlueprintResources/StandardMacros.IncrementInt` (`self.TurnNumber`))
          (:`  `
            (set `self.TurnNumber` _result_2))))
      (message `/Game/Cards/BI_CardUser.StartTurn` (`|GetArrayItem` (`self.Characters`) (`self.CharacterTurnIndex`))))))

(event `/Game/GameModes/BI_CardGameMode.CharacterDied`
  (params (Actor :type "Actor Object Reference"))
  (`KismetArrayLibrary.Array_RemoveItem` (`self.Characters`) Actor)
  (`KismetArrayLibrary.Array_RemoveItem` (`self.Enemies`) Actor))

(fn `GetAllEnemies`
  (returns (Enemies :type "Array of Actor Object Reference"))
  (return (`self.Enemies`)))

(fn `GetDefaultPawnClassForController`
  (params (InController :type "Controller Object Reference"))
  (returns (ReturnValue :type "Object Class Reference"))
  (bind _returnvalue (`parent.GetDefaultPawnClassForController` InController))
  (bind _selectedcharacterclass (message `/Game/GameModes/BI_CharacterSelection.GetSelectedCharacter` (`GameplayStatics.GetGameInstance`)))
  (if (`KismetSystemLibrary.IsValidClass` _selectedcharacterclass)
    (return _selectedcharacterclass)
    (else
      (return _returnvalue))))

(fn `GetTurnNumber`
  (returns (TurnNumber :type Integer))
  (return (`self.TurnNumber`)))

(fn `IsMyTurn`
  (params (Character :type "Actor Object Reference"))
  (returns (IsTurn :type Boolean))
  (return (== (`KismetArrayLibrary.Array_Find` (`self.Characters`) Character) (`self.CharacterTurnIndex`))))

(fn `UserConstructionScript`)